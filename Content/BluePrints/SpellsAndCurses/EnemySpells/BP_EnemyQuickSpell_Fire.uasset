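; Enemy fire quick spell that plays a short cast sound when it spawns.
; On hit, it deals impact damage and spawns a level 1 burn curse, attaches it to the receiver and begins it.
; A shield hit deals the same damage with a camera shake instead of the burn.
; When destroyed, it spawns an explosion effect and hit sound.
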(event `self.ReceiveBeginPlay`
  ;[1 1 1] Spawn
  (bind _returnvalue (`GameplayStatics.SpawnSoundAtLocation` "/Game/Audio/Magic/Fire_QuickSpellCast_CUE.Fire_QuickSpellCast_CUE" (`self.K2_GetActorLocation`) (struct) 1.0 1.0 0.0 null null false))
  (`AudioComponent.StopDelayed` _returnvalue 0.3))

(event `self.OnSpellHit`
  (params (curseReceiver :type "MythicismCharacter Object Reference"))
  ;[1 1 1] Hit
  (`MythicismCharacter.TakeDamage` curseReceiver (`self.ImpactDamage`) "HealthDamageType" null)
  (bind _returnvalue (`|SpawnActorFromClass` "/Game/BluePrints/SpellsAndCurses/Curses/BP_BurnCurse_lvl1.BP_BurnCurse_lvl1_C" (`KismetMathLibrary.MakeTransform` (0.0 0.0 0.0) (struct) (1.0 1.0 1.0)) "Undefined" "OverrideRootScale" null null))
  (set `Curse.curseReceiver` curseReceiver _returnvalue)
  (`self.K2_AttachToActor` _returnvalue curseReceiver "None" "KeepRelative" "KeepRelative" "KeepRelative" true)
  (`Curse.BeginCurse` _returnvalue))

(event `self.OnSpellHitShield`
  (params (curseReceiver :type "Shield Object Reference"))
  ;[1 1 1] Hit
  (`Shield.TakeDamage` curseReceiver (`self.ImpactDamage`) "HealthDamageType" null)
  (`GameplayStatics.PlayWorldCameraShake` "/Game/BluePrints/UI/BP_Boss_LightningShake.BP_Boss_LightningShake_C" (`self.K2_GetActorLocation` self) 0.0 1000.0 1.0 true))

(event `self.ReceiveDestroyed`
  (bind _returnvalue (`self.K2_GetActorLocation`))
  ;[1 1 1] Destroyed
  (`GameplayStatics.SpawnEmitterAtLocation` "/Game/Particles/P_Explosion.P_Explosion" _returnvalue (struct) (0.6 0.6 0.6))
  (`GameplayStatics.SpawnSoundAtLocation` "/Game/Audio/Magic/Fire_QuickSpellHit_CUE.Fire_QuickSpellHit_CUE" _returnvalue (struct) 1.0 1.0 0.0 null null))

(fn `UserConstructionScript`)