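; Boss tornado spell projectile that homes in on the player and deals impact damage.
; On spawn it adds a scene component to the player as the homing target and attaches a five-second wind sound to it, overriding Find Homing Target as empty.
; Normal and shield hits both apply the same health damage, with an impact sound and radial camera shake.
; Destruction spawns a hit particle effect.
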(event `self.ReceiveBeginPlay`
  (bind _returnvalue (`GameplayStatics.SpawnSoundAtLocation` "/Game/Audio/Magic/LifeDrain_QuickSpellHit_PLACEHOLDER.LifeDrain_QuickSpellHit_PLACEHOLDER" (`self.K2_GetActorLocation`) (struct) 1.0 0.0 0.0 null null false))
  (`AudioComponent.StopDelayed` _returnvalue 0.2)
  (bind _returnvalue_2 (`AddComponent|NODE_AddSceneComponent-0` :`self` (`GameplayStatics.GetPlayerCharacter` 0)))
  (set `ProjectileMovementComponent.HomingTargetComponent` _returnvalue_2 (`self.projectileMovement`))
  (bind _returnvalue_3 (`GameplayStatics.SpawnSoundAttached` "/Game/Audio/BossSounds/Wind_Boss_Noise_Cue.Wind_Boss_Noise_Cue" _returnvalue_2 "None" (0.0 0.0 0.0) (struct) "KeepRelativeOffset" false 1.0 1.0 0.0 null null))
  (`KismetSystemLibrary.Delay` 5.0)
  (`AudioComponent.Stop` _returnvalue_3)
  (`ActorComponent.K2_DestroyComponent` _returnvalue_3))

(event `self.OnSpellHit`
  (params (curseReceiver :type "MythicismCharacter Object Reference"))
  (bind _returnvalue (`self.K2_GetActorLocation`))
  (bind _returnvalue_2 (`GameplayStatics.SpawnSoundAtLocation` "/Game/Audio/UI/Inventory/541480__eminyildirim__magic-lighting-spell-impact-punch.541480__eminyildirim__magic-lighting-spell-impact-punch" _returnvalue (struct) 1.0 1.0 0.0 null null))
  (`AudioComponent.StopDelayed` _returnvalue_2 0.5)
  (`MythicismCharacter.TakeDamage` curseReceiver (`self.ImpactDamage`) "HealthDamageType" null)
  (`GameplayStatics.PlayWorldCameraShake` "/Game/BluePrints/UI/BP_Boss_LightningShake.BP_Boss_LightningShake_C" _returnvalue 0.0 1500.0 1.0 true :!label _label))

(event `self.OnSpellHitShield`
  (params (curseReceiver :type "Shield Object Reference"))
  (bind _returnvalue (`GameplayStatics.SpawnSoundAtLocation` "/Game/Audio/UI/Inventory/541480__eminyildirim__magic-lighting-spell-impact-punch.541480__eminyildirim__magic-lighting-spell-impact-punch" (`self.K2_GetActorLocation`) (struct) 1.0 1.0 0.0 null null))
  (`AudioComponent.StopDelayed` _returnvalue 0.5)
  (`Shield.TakeDamage` curseReceiver (`self.ImpactDamage`) "HealthDamageType" null)
  (goto _label))

(event `self.ReceiveDestroyed`
  (`GameplayStatics.SpawnEmitterAtLocation` "/Game/Particles/FXVarietyPack/P_ky_hit1.P_ky_hit1" (`self.K2_GetActorLocation`)))

(fn `Find Homing Target`)

(fn `UserConstructionScript`)