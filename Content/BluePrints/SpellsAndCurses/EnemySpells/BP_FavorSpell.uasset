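; BP_FavorSpell is an enemy spell projectile that homes on the player and adds favor through the game mode when it lands.
; On BeginPlay it plays a cast sound and sets the homing target to a scene component it adds to player character 0.
; SetFavorAmount sets the favor value, which spell hits and shield hits both pass to ThirdPersonGameMode's AddFavor, so shields do not block it.
; FindHomingTarget is left empty.
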(event `self.ReceiveBeginPlay`
  (`GameplayStatics.SpawnSoundAtLocation` "/Game/Audio/Magic/Favor_QuickSpellCast_CUE.Favor_QuickSpellCast_CUE" (`self.K2_GetActorLocation`) (struct) 1.0 1.0 0.0 null null false)
  (bind _returnvalue (`AddComponent|NODE_AddSceneComponent-0` :`self` (`GameplayStatics.GetPlayerCharacter` 0)))
  (set `ProjectileMovementComponent.HomingTargetComponent` _returnvalue (`self.projectileMovement`)))

(event `self.OnSpellHit`
  (params (curseReceiver :type "MythicismCharacter Object Reference"))
  (bind _asthird_person_game_mode (cast `/Game/BluePrints/ThirdPersonCharacter/ThirdPersonGameMode` (`GameplayStatics.GetGameMode`) :!label _label))
  (`/Game/BluePrints/ThirdPersonCharacter/ThirdPersonGameMode.AddFavor` _asthird_person_game_mode (`self.FavorDamage`)))

(event `self.OnSpellHitShield`
  (params (curseReceiver :type "Shield Object Reference"))
  (goto _label))

(event `self.ReceiveDestroyed`)

(event `SetFavorAmount`
  (params (EnemyFavor :type "Float (double-precision)"))
  (set `self.FavorDamage` EnemyFavor))

(fn `Find Homing Target`)

(fn `UserConstructionScript`)