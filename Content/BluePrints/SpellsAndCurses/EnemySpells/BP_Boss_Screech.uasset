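; BP_Boss_Screech is a boss screech spell that damages what it hits and shakes nearby cameras.
; On spawn it plays a short cast sound and an attached electric noise, while a timeline scales up the screech particles.
; Direct and shield hits both apply the same impact damage and an epicenter-oriented camera shake.
; The noise stops shortly after scaling finishes, and destruction spawns a thunder-ball burst with a hit sound.
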(event `self.ReceiveBeginPlay`
  (bind _soundeffect (`self.SoundEffect`))
  (bind _returnvalue (`GameplayStatics.SpawnSoundAtLocation` "/Game/Audio/Magic/LifeDrain_QuickSpellHit_PLACEHOLDER.LifeDrain_QuickSpellHit_PLACEHOLDER" (`self.K2_GetActorLocation`) (struct) 1.0 0.0 0.0 null null false))
  (`AudioComponent.StopDelayed` _returnvalue 0.2)
  (bind _returnvalue_2 (`GameplayStatics.SpawnSoundAttached` "/Game/Audio/BossSounds/Electric_Boss_Noise_Cue.Electric_Boss_Noise_Cue" null "None" (0.0 0.0 0.0) (struct) "KeepRelativeOffset" false 1.0 1.0 0.0 null null))
  (set `self.SoundEffect` _returnvalue_2)
  (bind (_direction _spell_scale) (`Timeline|ScaleIncrease` :!via `PlayFromStart`)
    (:`Update`
      (`SceneComponent.SetWorldScale3D` (`self.ScreechParticles`) (`KismetMathLibrary.MakeVector` _spell_scale _spell_scale _spell_scale)))
    (:`Finished`
      (`KismetSystemLibrary.Delay` 2.0)
      (`AudioComponent.Stop` _soundeffect)
      (`ActorComponent.K2_DestroyComponent` _soundeffect))))

(event `self.OnSpellHit`
  (params (curseReceiver :type "MythicismCharacter Object Reference"))
  (`MythicismCharacter.TakeDamage` curseReceiver (`self.ImpactDamage`) "HealthDamageType" null)
  (`GameplayStatics.PlayWorldCameraShake` "/Game/BluePrints/UI/BP_Boss_LightningShake.BP_Boss_LightningShake_C" (`self.K2_GetActorLocation` self) 0.0 3000.0 1.0 true :!label _label))

(event `self.OnSpellHitShield`
  (params (curseReceiver :type "Shield Object Reference"))
  (`Shield.TakeDamage` curseReceiver (`self.ImpactDamage`) "HealthDamageType" null)
  (goto _label))

(event `self.ReceiveDestroyed`
  (bind _returnvalue (`self.K2_GetActorLocation`))
  (`GameplayStatics.SpawnEmitterAtLocation` "/Game/Particles/FXVarietyPack/P_ky_ThunderBallHit.P_ky_ThunderBallHit" _returnvalue)
  (`GameplayStatics.SpawnSoundAtLocation` "/Game/Audio/Magic/Fire_QuickSpellHit_CUE.Fire_QuickSpellHit_CUE" _returnvalue (struct) 1.0 1.0 0.0 null null))

(fn `UserConstructionScript`)