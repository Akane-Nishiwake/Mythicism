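; BP_BurnCurse_lvl2 is a level 2 burn curse actor that deals damage over time to its CurseReceiver.
; The Curse event applies fixed health-type damage, then re-calls itself after a one-second delay for up to twelve seconds from CurseStartTime.
; When time runs out or the receiver becomes invalid, RemoveCurse prints a message and destroys the actor.
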(event `self.Curse`
  ;[1 1 1] Curse
  (if (and (< (`KismetSystemLibrary.GetGameTimeInSeconds`) (+ (`self.curseStartTime`) 12.0)) (`KismetSystemLibrary.IsValid` (`self.curseReceiver`)))
    (`MythicismCharacter.TakeDamage` (`self.curseReceiver`) 30.0 "HealthDamageType" null)
    (`KismetSystemLibrary.Delay` 1.0)
    (`self.Curse`)
    (else
      (`self.RemoveCurse`))))

(event `self.RemoveCurse`
  ;[1 1 1] Remove Curse
  (`KismetSystemLibrary.PrintString` "Curse removed" true true (struct :`R` 0.271933 :`B` 1.0 :`A` 1.0) 10.0)
  (`self.K2_DestroyActor`))

(fn `UserConstructionScript`)