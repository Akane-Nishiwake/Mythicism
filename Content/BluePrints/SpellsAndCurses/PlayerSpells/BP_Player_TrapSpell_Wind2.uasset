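; Player wind trap spell that damages whatever it hits and flings it upward with a randomized horizontal push.
; On spawn it plays a wind sound and grows via a scale timeline, then shrinks after a fixed lifetime and destroys itself when the reverse finishes.
; Tick keeps the timeline playing or reversing according to the SpellIsGrowing flag.
; OnSpellHit applies health damage and the launch to the receiver.
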(event `self.ReceiveBeginPlay`
  ;[1 1 1] Spell spawning and despawning
  (`|ExecutionSequence`
    (:`then_0`
      (bind _returnvalue (`GameplayStatics.SpawnSoundAtLocation` "/Game/Audio/BossSounds/Wind_Boss_Noise_Cue.Wind_Boss_Noise_Cue" (`self.K2_GetActorLocation`) (struct) 1.0 1.0 0.0 null null))
      (`KismetSystemLibrary.Delay` 3.0)
      (`ActorComponent.K2_DestroyComponent` _returnvalue))
    (:`then_1`
      (bind (_direction _scale) (`Timeline|ScaleTimeline` :`NewTime` (stale `self.ReceiveTick` DeltaSeconds) :!via `PlayFromStart` :!label _label)
        (:`Update`
          (`SceneComponent.SetWorldScale3D` (`self.root`) (`KismetMathLibrary.MakeVector` _scale _scale _scale)))
        (:`Finished`
          (if (not (`self.SpellIsGrowing?`))
            (`self.K2_DestroyActor`)
            (`ActorComponent.K2_DestroyComponent` (stale `ShrinkSpell` _returnvalue))))))
    (:`then_2`
      (`KismetSystemLibrary.Delay` 20.0)
      (`self.ShrinkSpell`))))

(event `self.ReceiveTick`
  (params (DeltaSeconds :type "Float (single-precision)"))
  ;[1 1 1] Spell spawning and despawning
  (if (`self.SpellIsGrowing?`)
    (goto _label)
    (else
      (goto _label :!via `Reverse`))))

(event `ShrinkSpell`
  ;[1 1 1] Spell spawning and despawning
  (set `self.SpellIsGrowing?` false)
  (bind _returnvalue (`GameplayStatics.SpawnSoundAtLocation` "/Game/Audio/BossSounds/Wind_Boss_Noise_Cue.Wind_Boss_Noise_Cue" (`self.K2_GetActorLocation`) (struct) 1.0 1.0 0.0 null null))
  (goto _label :!via `ReverseFromEnd`))

(event `self.OnSpellHit`
  (params (curseReceiver :type "MythicismCharacter Object Reference"))
  (`MythicismCharacter.TakeDamage` curseReceiver 25.0 "HealthDamageType" null)
  (`Character.LaunchCharacter` curseReceiver (`KismetMathLibrary.MakeVector` (`KismetMathLibrary.RandomFloatInRange` 500.0 1000.0) (`KismetMathLibrary.RandomFloatInRange` 500.0 1000.0) 1000.0) false false))

(fn `UserConstructionScript`)