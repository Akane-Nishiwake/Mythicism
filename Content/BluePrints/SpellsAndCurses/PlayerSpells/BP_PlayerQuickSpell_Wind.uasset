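; BP_PlayerQuickSpell_Wind is the player's quick wind spell, a short-lived actor that damages and pushes back what it hits.
; On spawn it plays a briefly cut impact sound and disables collision on its shockwave and sphere components.
; HitCollider overlaps apply health damage and an animation interrupt to any MythicismCharacter, plus slightly upward knockback along the collider's facing for BP_Enemy_1_Character.
; Tick counts Lifetime down from Duration and destroys the actor.
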(event `self.ReceiveBeginPlay`
  (bind _returnvalue (`GameplayStatics.SpawnSoundAtLocation` "/Game/Audio/UI/Inventory/541480__eminyildirim__magic-lighting-spell-impact-punch.541480__eminyildirim__magic-lighting-spell-impact-punch" (`self.K2_GetActorLocation`) (struct) 1.0 1.0 0.0 null null false))
  (`AudioComponent.StopDelayed` _returnvalue 0.3)
  (set `self.Lifetime` (`self.Duration`))
  (`PrimitiveComponent.SetCollisionEnabled` (`self.P_ky_shotShockwave`) "NoCollision")
  (`PrimitiveComponent.SetCollisionEnabled` (`self.Sphere`) "NoCollision"))

(event `self.hitCollider.OnComponentBeginOverlap`
  (params (OverlappedComponent :type "PrimitiveComponent Object Reference") (OtherActor :type "Actor Object Reference") (OtherComp :type "PrimitiveComponent Object Reference") (OtherBodyIndex :type Integer) (bFromSweep :type Boolean) (SweepResult :type "HitResult Structure (by ref)"))
  ;[1 1 1] Spell hit
  (bind _asmythicism_character (cast `MythicismCharacter` OtherActor))
  (`MythicismCharacter.TakeDamage` _asmythicism_character 50.0 "HealthDamageType" null)
  (message `/Game/BluePrints/MythicismPlayer/BPI_AnimationTriggerable.Interrupt` (`SkeletalMeshComponent.GetAnimInstance` (`Character.Mesh` _asmythicism_character)))
  (bind _asbp_enemy_1_character (cast `/Game/BluePrints/Enemies/BP_Enemy_1_Character` OtherActor))
  (`/Game/BluePrints/Enemies/BP_Enemy_1_Character.TakeKnockBack` _asbp_enemy_1_character (`KismetMathLibrary.GreaterGreater_VectorRotator` (1.0 0.0 0.25) (`SceneComponent.K2_GetComponentRotation` (`self.hitCollider`))) (`self.PushBackForce`)))

(event `self.ReceiveDestroyed`
  ;[1 1 1] On Destroy
)

(event `self.ReceiveTick`
  (params (DeltaSeconds :type "Float (single-precision)"))
  ;[1 1 1] Tick
  (bind _output_get (set `self.Lifetime` (- (`self.Lifetime`) DeltaSeconds)))
  (if (not (> _output_get 0.0))
    (`self.K2_DestroyActor`)))

(fn `UserConstructionScript`)