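; BP_PlayerQuickSpell_Fire is the player's quick fire spell, dealing impact damage and setting its target burning.
; A briefly played cast sound marks its spawn.
; Spell hits and shield hits both apply health damage, then spawn a level 1 burn curse actor, attach it to the receiver and begin it.
; Destruction spawns a scaled-down explosion effect and hit sound at the spell's location.
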(event `self.ReceiveBeginPlay`
  ;[1 1 1] Spawn
  (bind _returnvalue (`GameplayStatics.SpawnSoundAtLocation` "/Game/Audio/Magic/Fire_QuickSpellCast_CUE.Fire_QuickSpellCast_CUE" (`self.K2_GetActorLocation`) (struct) 1.0 1.0 0.0 null null false))
  (`AudioComponent.StopDelayed` _returnvalue 0.3))

(event `self.OnSpellHit`
  (params (curseReceiver :type "MythicismCharacter Object Reference"))
  ;[1 1 1] Impact
  (`MythicismCharacter.TakeDamage` curseReceiver (`self.ImpactDamage`) "HealthDamageType" null)
  (bind _returnvalue (`|SpawnActorFromClass` "/Game/BluePrints/SpellsAndCurses/Curses/BP_BurnCurse_lvl1.BP_BurnCurse_lvl1_C" (`KismetMathLibrary.MakeTransform` (0.0 0.0 0.0)) "Undefined" "OverrideRootScale" null null :!label _label))
  (set `Curse.curseReceiver` curseReceiver _returnvalue)
  (`self.K2_AttachToActor` _returnvalue curseReceiver "None" "KeepRelative" "KeepRelative" "KeepRelative" true)
  (`Curse.BeginCurse` _returnvalue))

(event `self.OnSpellHitShield`
  (params (curseReceiver :type "Shield Object Reference"))
  ;[1 1 1] Impact
  (`Shield.TakeDamage` curseReceiver (`self.ImpactDamage`) "HealthDamageType" null)
  (goto _label))

(event `self.ReceiveDestroyed`
  (bind _returnvalue (`self.K2_GetActorLocation`))
  ;[1 1 1] On destroy
  (`GameplayStatics.SpawnEmitterAtLocation` "/Game/Particles/P_Explosion.P_Explosion" _returnvalue (struct) (0.6 0.6 0.6))
  (`GameplayStatics.SpawnSoundAtLocation` "/Game/Audio/Magic/Fire_QuickSpellHit_CUE.Fire_QuickSpellHit_CUE" _returnvalue (struct) 1.0 1.0 0.0 null null))

(fn `UserConstructionScript`)