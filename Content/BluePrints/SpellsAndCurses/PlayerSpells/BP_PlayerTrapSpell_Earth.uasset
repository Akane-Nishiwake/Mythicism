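; BP_PlayerTrapSpell_Earth is a player earth trap spell that grows into an area, drains its victims, then shrinks away.
; A scale timeline drives growth and, after 45 seconds, the shrink that ends in destruction.
; Tick runs PerformCurses, periodically damaging every curse receiver and healing the caster per hit.
; Enemy_1 characters hit by the spell become more vulnerable to fall damage until they leave the collider, which resets threshold and mass-based multiplier.
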(event `self.ReceiveBeginPlay`
  ;[1 1 1] Spell spawning and despawning
  (`|ExecutionSequence`
    (:`then_0`
      (bind (_direction _scale) (`Timeline|ScaleTimeline` :`NewTime` (stale `self.ReceiveTick` DeltaSeconds) :!via `PlayFromStart` :!label _label)
        (:`Update`
          (`SceneComponent.SetWorldScale3D` (`self.root`) (`KismetMathLibrary.MakeVector` _scale _scale _scale)))
        (:`Finished`
          (if (not (`self.SpellIsGrowing?`))
            (`self.K2_DestroyActor`)))))
    (:`then_1`
      (bind _returnvalue (`GameplayStatics.SpawnSoundAtLocation` "/Game/Audio/Magic/mixkit-shot-light-energy-flowing-extra-short.mixkit-shot-light-energy-flowing-extra-short" (`self.K2_GetActorLocation`) (struct) 1.0 -1.0 0.0 null null false))
      (`AudioComponent.StopDelayed` _returnvalue 1.2)
      (bind _returnvalue_2 (`GameplayStatics.SpawnSoundAtLocation` "/Game/Audio/Fire01.Fire01" (`self.K2_GetActorLocation`) (struct) 1.0 2.0 0.0 null null false))
      (`AudioComponent.StopDelayed` _returnvalue_2 8.0)
      (bind _returnvalue_3 (`GameplayStatics.SpawnSoundAtLocation` "/Game/Audio/Fire_Sparks01.Fire_Sparks01" (`self.K2_GetActorLocation`) (struct) 1.0 -1.0 0.0 null null))
      (`AudioComponent.StopDelayed` _returnvalue_3 1.0))
    (:`then_2`
      (`KismetSystemLibrary.Delay` 45.0)
      (`self.ShrinkSpell`))))

(event `self.ReceiveTick`
  (params (DeltaSeconds :type "Float (single-precision)"))
  ;[1 1 1] Spell spawning and despawning
  (`self.PerformCurses`)
  (if (`self.SpellIsGrowing?`)
    (goto _label)
    (else
      (goto _label :!via `Reverse`))))

(event `ShrinkSpell`
  ;[1 1 1] Spell spawning and despawning
  (set `self.SpellIsGrowing?` false)
  (goto _label :!via `ReverseFromEnd`))

(event `self.OnSpellHit`
  (params (curseReceiver :type "MythicismCharacter Object Reference"))
  ;[1 1 1] Enter and exit circle
  (bind _asbp_enemy_1_character (cast `/Game/BluePrints/Enemies/BP_Enemy_1_Character` curseReceiver))
  (set `/Game/BluePrints/Enemies/BP_Enemy_1_Character.FallDamageMultiplier` 2.0 _asbp_enemy_1_character)
  (set `/Game/BluePrints/Enemies/BP_Enemy_1_Character.FallDamageVelocityThreshold` 200.0 _asbp_enemy_1_character))

(event `self.hitCollider.OnComponentEndOverlap`
  (params (OverlappedComponent :type "PrimitiveComponent Object Reference") (OtherActor :type "Actor Object Reference") (OtherComp :type "PrimitiveComponent Object Reference") (OtherBodyIndex :type Integer))
  ;[1 1 1] Enter and exit circle
  (bind _asbp_enemy_1_character (cast `/Game/BluePrints/Enemies/BP_Enemy_1_Character` OtherActor))
  (set `/Game/BluePrints/Enemies/BP_Enemy_1_Character.FallDamageMultiplier` (/ (`CharacterMovementComponent.Mass` (`Character.CharacterMovement` _asbp_enemy_1_character)) 100.0) _asbp_enemy_1_character)
  (set `/Game/BluePrints/Enemies/BP_Enemy_1_Character.FallDamageVelocityThreshold` 1500.0 _asbp_enemy_1_character))

(fn `PerformCurses`
  ;[1 1 1] Check if its time to curse
  (set `self.elapsedTime` (+ (`self.elapsedTime`) (`GameplayStatics.GetWorldDeltaSeconds`)))
  (if (and (>= (`self.elapsedTime`) 0.5) (`KismetSystemLibrary.IsValid` (`self.spellCaster`)))
    (set `self.elapsedTime` 0.0)
    (bind _result (`BlueprintSetLibrary.Set_ToArray` (`self.curseReceivers`)))
    (for _array_element _result
      ;[1 1 1] Curse
      (`MythicismCharacter.TakeDamage` _array_element 40.0 "HealthDamageType" null)
      (`MythicismCharacter.Heal` (`self.spellCaster`) 40.0 "HealthDamageType"))))

(fn `UserConstructionScript`)