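; Fire trap player spell that damages what it hits and applies a level 1 burn curse.
; A scale timeline grows the trap on spawn; after a fixed delay ShrinkSpell reverses it, and the actor is destroyed when it finishes, with Tick driving direction from SpellIsGrowing.
; OnSpellHit deals health damage, then spawns BP_BurnCurse_lvl1, attaches it to the receiver and starts it.
; Sound cues mark spawn, hit and despawn.
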(event `self.ReceiveBeginPlay`
  ;[1 1 1] Spell spawning and despawning
  (`|ExecutionSequence`
    (:`then_0`
      (`GameplayStatics.SpawnSoundAtLocation` "/Game/Audio/Magic/Fire_TrapSpellSpawn_CUE.Fire_TrapSpellSpawn_CUE" (`self.K2_GetActorLocation`) (struct) 1.0 1.0 0.0 null null))
    (:`then_1`
      (bind (_direction _scale) (`Timeline|ScaleTimeline` :`NewTime` (stale `self.ReceiveTick` DeltaSeconds) :!via `PlayFromStart` :!label _label)
        (:`Update`
          (`SceneComponent.SetWorldScale3D` (`self.root`) (`KismetMathLibrary.MakeVector` _scale _scale _scale)))
        (:`Finished`
          (if (not (`self.SpellIsGrowing?`))
            (`self.K2_DestroyActor`)))))
    (:`then_2`
      (`KismetSystemLibrary.Delay` 20.0)
      (`self.ShrinkSpell`))))

(event `self.ReceiveTick`
  (params (DeltaSeconds :type "Float (single-precision)"))
  ;[1 1 1] Spell spawning and despawning
  (if (`self.SpellIsGrowing?`)
    (goto _label)
    (else
      (goto _label :!via `Reverse`))))

(event `ShrinkSpell`
  ;[1 1 1] Spell spawning and despawning
  (set `self.SpellIsGrowing?` false)
  (`GameplayStatics.SpawnSoundAtLocation` "/Game/Audio/Magic/Fire_TrapSpellDespawn_CUE.Fire_TrapSpellDespawn_CUE" (`self.K2_GetActorLocation`) (struct) 1.0 1.0 0.0 null null)
  (goto _label :!via `ReverseFromEnd`))

(event `self.OnSpellHit`
  (params (curseReceiver :type "MythicismCharacter Object Reference"))
  (`MythicismCharacter.TakeDamage` curseReceiver 25.0 "HealthDamageType" null)
  (`GameplayStatics.SpawnSoundAtLocation` "/Game/Audio/Magic/Fire_TrapSpellEnter_CUE.Fire_TrapSpellEnter_CUE" (`self.K2_GetActorLocation`) (struct) 1.0 1.0 0.0 null null)
  (bind _returnvalue (`|SpawnActorFromClass` "/Game/BluePrints/SpellsAndCurses/Curses/BP_BurnCurse_lvl1.BP_BurnCurse_lvl1_C" (`KismetMathLibrary.MakeTransform` (0.0 0.0 0.0)) "Undefined" "OverrideRootScale" null null))
  (set `Curse.curseReceiver` curseReceiver _returnvalue)
  (`self.K2_AttachToActor` _returnvalue curseReceiver "None" "KeepRelative" "KeepRelative" "KeepRelative" true)
  (`Curse.BeginCurse` _returnvalue))

(fn `UserConstructionScript`)