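; Wind trap player spell that catches enemies, lifts and spins them, then hurls them away.
; A timeline scales the spell in, then after a delay releases victims, shrinks and destroys it.
; OnSpellHit ragdolls enemies without gravity and starts per-victim float timers.
; PerformCurses runs each tick, lifting and spinning victims until timers expire, then launching them along the camera direction captured at spawn.
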(event `self.ReceiveBeginPlay`
  ;[1 1 1] Spell spawning and despawning
  (set `self.Direction` (`self.GetActorForwardVector` (`GameplayStatics.GetPlayerCameraManager` 0)))
  (`|ExecutionSequence`
    (:`then_0`
      (bind (_direction _scale) (`Timeline|ScaleTimeline` :`NewTime` (stale `self.ReceiveTick` DeltaSeconds) :!via `PlayFromStart` :!label _label)
        (:`Update`
          (`SceneComponent.SetWorldScale3D` (`self.root`) (`KismetMathLibrary.MakeVector` _scale _scale _scale)))
        (:`Finished`
          (if (not (`self.SpellIsGrowing?`))
            (`self.K2_DestroyActor`)))))
    (:`then_1`
      (bind _returnvalue (`GameplayStatics.SpawnSoundAtLocation` "/Game/Audio/Magic/mixkit-shot-light-energy-flowing-extra-short.mixkit-shot-light-energy-flowing-extra-short" (`self.K2_GetActorLocation`) (struct) 1.0 -1.0 0.0 null null false))
      (`AudioComponent.StopDelayed` _returnvalue 1.2)
      (bind _returnvalue_2 (`GameplayStatics.SpawnSoundAtLocation` "/Game/Audio/Fire01.Fire01" (`self.K2_GetActorLocation`) (struct) 1.0 2.0 0.0 null null false))
      (`AudioComponent.StopDelayed` _returnvalue_2 8.0)
      (bind _returnvalue_3 (`GameplayStatics.SpawnSoundAtLocation` "/Game/Audio/Fire_Sparks01.Fire_Sparks01" (`self.K2_GetActorLocation`) (struct) 1.0 -1.0 0.0 null null))
      (`AudioComponent.StopDelayed` _returnvalue_3 1.0))
    (:`then_2`
      (`KismetSystemLibrary.Delay` 6.0)
      (`self.ReleaseVictims`)
      (`self.ShrinkSpell`))))

(event `self.ReceiveTick`
  (params (DeltaSeconds :type "Float (single-precision)"))
  ;[1 1 1] Spell spawning and despawning
  (for (_array_element _array_index) (`self.RecieverFloatTime`)
    (`KismetArrayLibrary.Array_Set` (`self.RecieverFloatTime`) _array_index (+ _array_element DeltaSeconds)))
  (`self.PerformCurses`)
  (if (`self.SpellIsGrowing?`)
    (goto _label)
    (else
      (goto _label :!via `Reverse`))))

(event `ShrinkSpell`
  ;[1 1 1] Spell spawning and despawning
  (set `self.SpellIsGrowing?` false)
  (goto _label :!via `ReverseFromEnd`))

(event `self.OnSpellHit`
  (params (curseReceiver :type "MythicismCharacter Object Reference"))
  (bind _charactermovement (`Character.CharacterMovement` curseReceiver))
  ;[1 1 1] Enter and exit circle
  (`BlueprintSetLibrary.Set_Add` (`self.curseReceivers`) curseReceiver)
  (`KismetArrayLibrary.Array_Add` (`self.RecieverFloatTime`))
  (bind _asbp_enemy_1_character (cast `/Game/BluePrints/Enemies/BP_Enemy_1_Character` curseReceiver))
  (set `CharacterMovementComponent.GravityScale` 0.0 _charactermovement)
  (`/Game/BluePrints/Enemies/BP_Enemy_1_Character.TakeKnockBack` _asbp_enemy_1_character (0.0 0.0 1.0) (`CharacterMovementComponent.Mass` _charactermovement))
  (`/Game/BluePrints/Enemies/BP_Enemy_1_Character.BeginRagdoll` _asbp_enemy_1_character)
  (`PrimitiveComponent.SetPhysicsLinearVelocity` (`Character.CapsuleComponent` curseReceiver) (0.0 0.0 0.0) false "None"))

(event `self.hitCollider.OnComponentEndOverlap`
  (params (OverlappedComponent :type "PrimitiveComponent Object Reference") (OtherActor :type "Actor Object Reference") (OtherComp :type "PrimitiveComponent Object Reference") (OtherBodyIndex :type Integer))
  ;[1 1 1] Enter and exit circle
)

(event `ReleaseVictims`
  (bind _result (`BlueprintSetLibrary.Set_ToArray` (`self.curseReceivers`)))
  (for _array_element _result
    (`/Engine/EditorBlueprintResources/StandardMacros.IsValid` _array_element
      (:`Is Valid`
        (set `CharacterMovementComponent.GravityScale` 1.0 (`Character.CharacterMovement` _array_element))))))

(fn `PerformCurses`
  (bind _recieverfloattime (`self.RecieverFloatTime`))
  ;[1 1 1] Stage 1
  (bind _result (`BlueprintSetLibrary.Set_ToArray` (`self.curseReceivers`)))
  (for (_array_element _array_index) _result
    (`/Engine/EditorBlueprintResources/StandardMacros.IsValid` _array_element
      (:`Is Valid`
        (if (`KismetArrayLibrary.Array_IsValidIndex` _recieverfloattime _array_index)
          (if (> (`|GetArrayItem` _recieverfloattime _array_index) (`self.FloatTime`))
            (`KismetArrayLibrary.Array_Remove` (`self.RecieverFloatTime`) _array_index)
            (`BlueprintSetLibrary.Set_Remove` (`self.curseReceivers`) _array_element)
            (bind _asbp_enemy_1_character (cast `/Game/BluePrints/Enemies/BP_Enemy_1_Character` _array_element))
            (`/Game/BluePrints/Enemies/BP_Enemy_1_Character.TakeKnockBack` _asbp_enemy_1_character (+ (`self.Direction`) (0.0 0.0 0.25)) (`self.Pushback`))
            (bind _charactermovement (`Character.CharacterMovement` _array_element))
            (set `CharacterMovementComponent.GravityScale` 1.0 _charactermovement)
            (`PrimitiveComponent.AddTorqueInDegrees` (`Character.Mesh` _array_element) (0.0 0.0 2000001.0) "None" true)
            (else
              (`CharacterMovementComponent.SetMovementMode` _charactermovement "MOVE_Falling" 0)
              (bind _asbp_enemy_1_character_2 (cast `/Game/BluePrints/Enemies/BP_Enemy_1_Character` _array_element))
              (`/Game/BluePrints/Enemies/BP_Enemy_1_Character.TakeKnockBack` _asbp_enemy_1_character_2 (0.0 0.0 1.0) (/ (`self.FloatForce`) 2.25))
              (bind _mesh (`Character.Mesh` _array_element))
              (`PrimitiveComponent.SetPhysicsAngularVelocityInDegrees` _mesh (0.0 0.0 4000.0) true "None")
              (bind _returnvalue (`PrimitiveComponent.GetPhysicsLinearVelocity` _mesh "None"))
              (`PrimitiveComponent.SetPhysicsLinearVelocity` _mesh (`KismetMathLibrary.MakeVector` 0.0 0.0 (`KismetMathLibrary.FMin` (.z _returnvalue) 20.0)) false "None"))))))))

(fn `UserConstructionScript`)