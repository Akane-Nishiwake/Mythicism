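; Player quick-spell actor for Life Drain that damages what it hits and heals its caster.
; On hit, if the caster is still valid, it deals health damage to the curse receiver and heals the caster by the same amount.
; It plays a briefly cut-off cast sound on spawn, then a hit particle effect and sound when destroyed.
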(event `self.ReceiveBeginPlay`
  (bind _returnvalue (`GameplayStatics.SpawnSoundAtLocation` "/Game/Audio/Magic/LifeDrain_QuickSpellCast_CUE.LifeDrain_QuickSpellCast_CUE" (`self.K2_GetActorLocation`) (struct) 1.0 1.0 0.0 null null false))
  (`AudioComponent.StopDelayed` _returnvalue 0.3))

(event `self.OnSpellHit`
  (params (curseReceiver :type "MythicismCharacter Object Reference"))
  ;[1 1 1] Spell hit
  (if (`KismetSystemLibrary.IsValid` (`self.spellCaster`))
    (`MythicismCharacter.TakeDamage` curseReceiver 100.0 "HealthDamageType" null)
    (`MythicismCharacter.Heal` (`self.spellCaster`) 100.0 "HealthDamageType")))

(event `self.ReceiveDestroyed`
  (bind _returnvalue (`self.K2_GetActorLocation`))
  ;[1 1 1] On Destroy
  (`GameplayStatics.SpawnEmitterAtLocation` "/Game/Particles/FXVarietyPack/P_ky_LifeDrainlHit.P_ky_LifeDrainlHit" _returnvalue (struct) (0.6 0.6 0.6))
  (`GameplayStatics.PlaySoundAtLocation` "/Game/Audio/Magic/LifeDrain_QuickSpellHit_CUE.LifeDrain_QuickSpellHit_CUE" _returnvalue (struct) 1.0 1.0 0.0 null null null))

(fn `UserConstructionScript`)