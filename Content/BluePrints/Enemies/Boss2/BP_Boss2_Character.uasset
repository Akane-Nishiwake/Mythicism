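; Boss 2 enemy character that handles its health bar, damage reactions and death.
; On damage it spawns a blood decal, plays a physical-animation hit reaction and sounds, reveals the updated health bar, and turns to the player on the first hit via a timeline.
; On death it disables movement and capsule collision, plays a random death animation, decrements the game mode's enemy count, destroys itself and awards player currency.
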(event `self.ReceiveBeginPlay`
  ;[1 1 1] Set Enemy Health
  (bind _asenemy_health (cast `/Game/BluePrints/UI/Enemy/EnemyHealth` (`WidgetComponent.GetWidget` (`self.HealthBar`))))
  (set `/Game/BluePrints/UI/Enemy/EnemyHealth.MaxHealth` (`CharacterAttributesComponent.maxHealth` (`self.attributes`)) _asenemy_health)
  (set `/Game/BluePrints/UI/Enemy/EnemyHealth.Health` (`CharacterAttributesComponent.health` (`self.attributes`)) _asenemy_health)
  (`Widget.SetVisibility` _asenemy_health "Hidden"))

(event `self.OnTakeDamage`
  (params (amount :type "Float (single-precision)") (damageType :type "EDamageTypes Enum (by ref)" :default "HealthDamageType"))
  (bind _returnvalue (`self.K2_GetActorLocation`))
  (bind _capsulecomponent (`self.CapsuleComponent`))
  (bind _returnvalue_2 (`WidgetComponent.GetWidget` (`self.HealthBar`)))
  (bind (_returnvalue_roll _returnvalue_pitch _returnvalue_yaw) (`KismetMathLibrary.BreakRotator` (`SceneComponent.K2_GetComponentRotation` _capsulecomponent)))
  (bind (_returnvalue_roll_2 _returnvalue_pitch_2 _returnvalue_yaw_2) (`KismetMathLibrary.BreakRotator` (`KismetMathLibrary.FindLookAtRotation` (`SceneComponent.K2_GetComponentLocation` _capsulecomponent) (`SceneComponent.K2_GetComponentLocation` (`Character.Mesh` (`GameplayStatics.GetPlayerCharacter` 0))))))
  ;[1 1 1] Enemy Takes Damage
  (`|SpawnActorFromClass` "/Game/Materials/WeaponTrails/BP_BloodDecal.BP_BloodDecal_C" (`KismetMathLibrary.MakeTransform` (`SceneComponent.K2_GetComponentLocation` (`self.Mesh`)) (`KismetMathLibrary.MakeRotator` 0.0 0.0 (`KismetMathLibrary.RandomFloatInRange` 0.0 360.0))) "Undefined" "OverrideRootScale" null null)
  (`/Game/BluePrints/Enemies/BP_PhysicalAnimComp.HitReaction` (`self.BP_PhysicalAnimComp`))
  (bind _asenemy_health (cast `/Game/BluePrints/UI/Enemy/EnemyHealth` _returnvalue_2))
  (set `/Game/BluePrints/UI/Enemy/EnemyHealth.Health` (`CharacterAttributesComponent.health` (`self.attributes`)) _asenemy_health)
  (`Widget.SetVisibility` _returnvalue_2 "Visible")
  (`GameplayStatics.SpawnSoundAtLocation` "/Game/Audio/Impact/sfx_hit1.sfx_hit1" (`self.K2_GetActorLocation`) (struct) 0.5 2.0 0.0 null null)
  (switch `int` (`KismetMathLibrary.RandomInteger` 3)
    (:`Default`
      (`GameplayStatics.SpawnSoundAtLocation` "/Game/Audio/VoicesPack_2/MonsterDeath.MonsterDeath" _returnvalue (struct) 0.75 1.0 0.0 null null :!label _label))
    (:`0`
      (goto _label))
    (:`1`
      (`GameplayStatics.SpawnSoundAtLocation` "/Game/Audio/VoicesPack_2/MonsterPain.MonsterPain" _returnvalue (struct) 0.75 1.0 0.0 null null))
    (:`2`
      (`GameplayStatics.SpawnSoundAtLocation` "/Game/Audio/VoicesPack_2/MonsterPain_01.MonsterPain_01" _returnvalue (struct) 0.75 1.0 0.0 null null)))
  (`/Engine/EditorBlueprintResources/StandardMacros.DoOnce` false
    (:`Completed`
      (bind (_direction _value) (`Timeline|Timeline_0` :!via `PlayFromStart`)
        (:`Update`
          (`SceneComponent.K2_SetWorldRotation` _capsulecomponent (`KismetMathLibrary.MakeRotator` _returnvalue_roll _returnvalue_pitch (`KismetMathLibrary.Lerp` _returnvalue_yaw _returnvalue_yaw_2 _value)) false false))))))

(event `self.OnDie`
  (bind _mesh (`self.Mesh`))
  ;[1 1 1] Enemy Death
  (set `CharacterAttributesComponent.isInvincible` true (`self.attributes`))
  (`ActorComponent.K2_DestroyComponent` (`self.CameraTarget`))
  (bind _asenemy_health (cast `/Game/BluePrints/UI/Enemy/EnemyHealth` (`WidgetComponent.GetWidget` (`self.HealthBar`))))
  (set `/Game/BluePrints/UI/Enemy/EnemyHealth.Health` (`CharacterAttributesComponent.health` (`self.attributes`)) _asenemy_health)
  (`/Engine/EditorBlueprintResources/StandardMacros.DoOnce` false
    (:`Completed`
      (set `self.bUseControllerRotationYaw` false)
      (`CharacterMovementComponent.DisableMovement` (`self.CharacterMovement`))
      (`PrimitiveComponent.SetCollisionEnabled` (`self.CapsuleComponent`) "NoCollision")
      (`PrimitiveComponent.SetCollisionResponseToChannel` (`self.Mesh`) "ECC_PhysicsBody" "ECR_Ignore")
      (if (> (`KismetMathLibrary.RandomInteger` 2) 0)
        (`SkeletalMeshComponent.PlayAnimation` _mesh "/Game/Animations/ProSwordAndShield/swordandshielddeath_2_4UE4.swordandshielddeath_2_4UE4" false)
        (else
          (`SkeletalMeshComponent.PlayAnimation` _mesh "/Game/Animations/ProSwordAndShield/swordandshielddeath4UE4.swordandshielddeath4UE4" false)))
      (`KismetSystemLibrary.Delay` 2.0)
      (`PrimitiveComponent.SetSimulatePhysics` _mesh false)
      (bind _asthird_person_game_mode (cast `/Game/BluePrints/ThirdPersonCharacter/ThirdPersonGameMode` (`GameplayStatics.GetGameMode`))
        (:`then`
          (set `/Game/BluePrints/ThirdPersonCharacter/ThirdPersonGameMode.NumberOfEnemies` (- (`/Game/BluePrints/ThirdPersonCharacter/ThirdPersonGameMode.NumberOfEnemies` _asthird_person_game_mode) 1) _asthird_person_game_mode)
          (`KismetSystemLibrary.Delay` 3.0)
          (`self.K2_DestroyActor`)
          (bind _asbp_mythicism_player (cast `/Game/BluePrints/MythicismPlayer/BP_MythicismPlayer` (`GameplayStatics.GetPlayerCharacter` 0)))
          (set `MythicismPlayer.playerCurrency` (+ (`MythicismPlayer.playerCurrency` _asbp_mythicism_player) (`KismetMathLibrary.FTrunc` (`self.favorAmount`))) _asbp_mythicism_player))
        (:`CastFailed`
          (`KismetSystemLibrary.PrintString` "Cast failed"))))))

(fn `UserConstructionScript`)