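; Enemy component that adds physics-driven hit reactions to the upper body of Enemy_1 and Boss2 characters.
; On BeginPlay it adds a physical animation component to the owner and binds it to the character mesh.
; HitReaction, effective only on non-ragdolled Enemy_1 owners, simulates bodies from neck_01 down with a backward impulse.
; Tick counts down a stacking timer, sets a capped physics blend weight, then stops simulation and ticking.
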(event `self.ReceiveBeginPlay`
  ;[1 1 1] Setup Physical Animation
  (bind _returnvalue (`|AddComponentByClass` (`self.GetOwner`) "/Script/Engine.PhysicalAnimationComponent"))
  (set `self.PhysicalAnimationComponent` _returnvalue)
  (bind _asenemy (cast `Enemy` (`self.GetOwner`)))
  (bind _asbp_enemy_1_character (cast `/Game/BluePrints/Enemies/BP_Enemy_1_Character` _asenemy)
    (:`then`
      (bind _mesh (`Character.Mesh` _asbp_enemy_1_character))
      (`PhysicalAnimationComponent.SetSkeletalMeshComponent` (`self.PhysicalAnimationComponent`) _mesh)
      (set `self.Mesh` _mesh))
    (:`CastFailed`
      (bind _asbp_boss_2_character (cast `/Game/BluePrints/Enemies/Boss2/BP_Boss2_Character` _asenemy))
      (bind _mesh_2 (`Character.Mesh` _asbp_boss_2_character))
      (`PhysicalAnimationComponent.SetSkeletalMeshComponent` (`self.PhysicalAnimationComponent`) _mesh_2)
      (set `self.Mesh` _mesh_2))))

(event `HitReaction`
  (bind _mesh (`self.Mesh`))
  ;[1 1 1] Hit React
  (bind _asbp_enemy_1_character (cast `/Game/BluePrints/Enemies/BP_Enemy_1_Character` (`self.GetOwner` (`self.Mesh`))))
  (if (not (`/Game/BluePrints/Enemies/BP_Enemy_1_Character.Ragdolled` _asbp_enemy_1_character))
    (`self.SetComponentTickEnabled` true)
    (set `self.HitTimeRemaining` (+ 1.0 (`self.HitTimeRemaining`)))
    (`PhysicalAnimationComponent.ApplyPhysicalAnimationProfileBelow` (`self.PhysicalAnimationComponent`) "neck_01" "UpperBody" true false)
    (`SkeletalMeshComponent.SetAllBodiesBelowSimulatePhysics` _mesh "neck_01" true true)
    (set `self.Impulse` (* (`SceneComponent.GetForwardVector` _mesh) -5000.0))
    (`PrimitiveComponent.AddImpulse` _mesh (`self.Impulse`) "neck_01" true)))

(event `self.ReceiveTick`
  (params (DeltaSeconds :type "Float (single-precision)"))
  ;[1 1 1] Hit React Timer
  (set `self.HitTimeRemaining` (- (`KismetMathLibrary.FInterpTo` (`self.HitTimeRemaining`) 0.0 0.0 1.0) (* DeltaSeconds 1.0)))
  (if (<= (`self.HitTimeRemaining`) 0.0)
    (set `self.HitTimeRemaining` 0.0)
    (`SkeletalMeshComponent.SetAllBodiesBelowSimulatePhysics` (`self.Mesh`) "neck_01" false true)
    (`self.SetComponentTickEnabled` false)
    (else
      (`SkeletalMeshComponent.SetAllBodiesBelowPhysicsBlendWeight` (`self.Mesh`) "neck_01" (`KismetMathLibrary.FMin` (`self.HitTimeRemaining`) 0.2) false true))))