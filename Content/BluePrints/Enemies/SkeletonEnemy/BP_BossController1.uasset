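; BP_BossController1 is the AI controller for a boss enemy in the SkeletonEnemy folder, driving its behavior and player detection.
; On BeginPlay it runs the Boss_1_Tree1 behavior tree.
; Perception updates for actors whose first tag is "Player" set focus on that actor and write the sensed state and player reference to the blackboard.
; Focus is set even when the player is lost, and never cleared here.
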(event `self.ReceiveBeginPlay`
  ;[1 1 1] Run Behavior Tree
  (`self.RunBehaviorTree` "/Game/BluePrints/Enemies/SkeletonEnemy/Boss_1_Tree1.Boss_1_Tree1"))

(event `self.AIPerception.OnTargetPerceptionUpdated`
  (params (Actor :type "Actor Object Reference") (Stimulus :type "AIStimulus Structure"))
  ;[1 1 1] Sense Player
  (if (== (`|GetArrayItem` (`Actor.Tags` Actor)) "Player")
    (`self.K2_SetFocus` Actor)
    (`BlackboardComponent.SetValueAsBool` (`AIBlueprintHelperLibrary.GetBlackboard` null) "CanSeePlayer?" (`.bSuccessfullySensed` (break `AIStimulus` Stimulus)))
    (`BlackboardComponent.SetValueAsObject` (`AIBlueprintHelperLibrary.GetBlackboard` null) "playerCharacter" Actor)))

(fn `UserConstructionScript`)