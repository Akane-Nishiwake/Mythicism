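; AI controller for the dagger enemy that drives its behavior trees.
; On BeginPlay it starts DaggerEnemy_Tree and caches the player character.
; Perception updates for actors whose first tag is "Player" set focus on that actor and write sight state and the player reference to the Blackboard.
; Tick polls the player's health and switches once to PlayerKilledbehavior when it runs out.
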(event `self.ReceiveTick`
  (params (DeltaSeconds :type "Float (single-precision)"))
  ;[1 1 1] Check if player dead
  (if (<= (`CharacterAttributesComponent.health` (`MythicismCharacter.attributes` (`self.As BP Mythicism Player`))) 0.0)
    (`/Engine/EditorBlueprintResources/StandardMacros.DoOnce` false
      (:`Completed`
        (`self.RunBehaviorTree` "/Game/BluePrints/Enemies/DaggerEnemy/PlayerKilledbehavior.PlayerKilledbehavior")))))

(event `self.ReceiveBeginPlay`
  ;[1 1 1] Run Behavior Tree
  (`self.RunBehaviorTree` "/Game/BluePrints/Enemies/DaggerEnemy/DaggerEnemy_Tree.DaggerEnemy_Tree")
  (bind _asbp_mythicism_player (cast `/Game/BluePrints/MythicismPlayer/BP_MythicismPlayer` (`GameplayStatics.GetPlayerCharacter` 0)))
  (set `self.As BP Mythicism Player` _asbp_mythicism_player))

(event `self.AIPerception.OnTargetPerceptionUpdated`
  (params (Actor :type "Actor Object Reference") (Stimulus :type "AIStimulus Structure"))
  ;[1 1 1] Sense Player
  (if (== (`|GetArrayItem` (`Actor.Tags` Actor)) "Player")
    (`self.K2_SetFocus` Actor)
    (`BlackboardComponent.SetValueAsBool` (`AIBlueprintHelperLibrary.GetBlackboard` null) "CanSeePlayer?" (`.bSuccessfullySensed` (break `AIStimulus` Stimulus)))
    (`BlackboardComponent.SetValueAsObject` (`AIBlueprintHelperLibrary.GetBlackboard` null) "playerCharacter" Actor)))

(fn `UserConstructionScript`)