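; Enemy character with weapon and shield hands that reacts to damage, knockback, hitstop and falls.
; Damage updates the health bar widget, spawns blood and sound, turns it toward the player and flags its AI blackboard.
; Knockback launches it; landing or ragdoll impacts deal velocity-based damage, with the capsule following the pelvis while ragdolled.
; Death stops AI, animates, decrements the game mode's enemy count and spawns a favor pickup scaled by player stats.
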(event `self.ReceiveActorBeginOverlap`
  (params (OtherActor :type "Actor Object Reference")))

(event `RagdollCollideWithSurface`
  (params (Velocity :type "Vector Structure") (Normal :type "Vector Structure") (Gravity :type "Vector Structure" :default (0.0 0.0 -1.0)) (Force :type "Float (double-precision)"))
  (bind _returnvalue (* (`KismetMathLibrary.FMax` (- (`KismetMathLibrary.VSize` Velocity) (`self.RagdollVelocityThreshold`))) (`KismetMathLibrary.ClampAngle` (* (`KismetMathLibrary.Dot_VectorVector` Velocity Normal) -1.0) 0.0 1.0)))
  ;[1 1 1] Ragdoll Surface Collision
  (`KismetSystemLibrary.PrintString` (`KismetStringLibrary.Conv_DoubleToString` _returnvalue))
  (if (and (> _returnvalue 0.0) (> (`self.FallDamageTimer`) 0.1))
    (set `self.FallDamageTimer` 0.0)
    (`self.TakeDamage` (/ _returnvalue 2.0) "HealthDamageType" null)))

(event `BeginRagdoll`
  (bind _capsulecomponent (`self.CapsuleComponent`))
  (bind _childactor (`ChildActorComponent.ChildActor` (`self.weaponHand`)))
  (bind _childactor_2 (`ChildActorComponent.ChildActor` (`self.shieldHand`)))
  ;[1 1 1] Begin Ragdoll
  (set `self.Ragdolled` true)
  (`PrimitiveComponent.SetSimulatePhysics` (`self.Mesh`) true)
  (`PrimitiveComponent.SetCollisionEnabled` _capsulecomponent "NoCollision")
  (`PrimitiveComponent.SetEnableGravity` _capsulecomponent false)
  (`CharacterMovementComponent.SetMovementMode` (`self.CharacterMovement`) "MOVE_Falling" 0)
  (`/Engine/EditorBlueprintResources/StandardMacros.IsValid` _childactor
    (:`Is Valid`
      (`self.SetActorEnableCollision` _childactor false))
    (:`Is Not Valid`
      _))
  (`/Engine/EditorBlueprintResources/StandardMacros.IsValid` _childactor_2
    (:`Is Valid`
      (`self.SetActorEnableCollision` _childactor_2 false))))

(event `self.ReceiveTick`
  (params (DeltaSeconds :type "Float (single-precision)"))
  (if (`self.Ragdolled`)
    (`SceneComponent.K2_SetWorldLocation` (`self.CapsuleComponent`) (`SceneComponent.GetSocketLocation` (`self.Mesh`) "pelvis") false true)
    (set `self.FallDamageTimer` (+ (`self.FallDamageTimer`) DeltaSeconds))))

(event `EndRagdoll`
  (bind _capsulecomponent (`self.CapsuleComponent`))
  (bind _healthbar (`self.HealthBar`))
  (bind _capsulecomponent_2 (`self.CapsuleComponent`))
  (bind _childactor (`ChildActorComponent.ChildActor` (`self.weaponHand`)))
  (bind _childactor_2 (`ChildActorComponent.ChildActor` (`self.shieldHand`)))
  (`SceneComponent.K2_SetWorldLocation` _capsulecomponent (+ (`SceneComponent.K2_GetComponentLocation` (`self.Mesh`)) (0.0 0.0 20.0)) false true)
  (`PrimitiveComponent.SetEnableGravity` _capsulecomponent true)
  (`KismetSystemLibrary.Delay` 1.0)
  (`PrimitiveComponent.SetSimulatePhysics` (`self.Mesh`) false)
  (set `self.Ragdolled` false)
  (`SceneComponent.K2_AttachToComponent` (`self.Mesh`) (`self.CapsuleComponent`) "None" "KeepRelative" "KeepRelative" "KeepWorld" true)
  (`SceneComponent.K2_SetWorldLocation` _capsulecomponent_2 (+ (`SceneComponent.K2_GetComponentLocation` _capsulecomponent_2) (0.0 0.0 40.0)) false false)
  (`SceneComponent.K2_SetRelativeLocationAndRotation` (`self.Mesh`) (0.0 0.0 -95.0) (struct :`Yaw` 270.0) false false)
  (`SceneComponent.K2_AttachToComponent` (`self.HealthBar`) (`self.CapsuleComponent`) "None" "KeepRelative" "KeepRelative" "KeepWorld" true)
  (`SceneComponent.K2_SetRelativeLocationAndRotation` :`self` _healthbar :`NewLocation` (0.0 0.0 100.0) :`bTeleport` true)
  (`WidgetComponent.SetWidgetSpace` _healthbar "Screen")
  (`PrimitiveComponent.SetCollisionEnabled` (`self.CapsuleComponent`) "QueryOnly")
  (`/Engine/EditorBlueprintResources/StandardMacros.IsValid` _childactor
    (:`Is Valid`
      (`self.SetActorEnableCollision` _childactor true))
    (:`Is Not Valid`
      _))
  (`/Engine/EditorBlueprintResources/StandardMacros.IsValid` _childactor_2
    (:`Is Valid`
      (`self.SetActorEnableCollision` _childactor_2 true))))

(event `TakeKnockBack`
  (params (Direction :type "Vector Structure") (Magnitude :type "Float (double-precision)"))
  (bind _returnvalue (* Direction Magnitude))
  (bind _charactermovement (`self.CharacterMovement`))
  (if (`self.Ragdolled`)
    (`PrimitiveComponent.AddImpulseAtLocation` (`self.Mesh`) (* Direction Magnitude) (`self.K2_GetActorLocation`) "None")
    (else
      (bind _asenemy_health (cast `/Game/BluePrints/UI/Enemy/EnemyHealth` (`WidgetComponent.GetWidget` (`self.HealthBar`))))
      (set `/Game/BluePrints/UI/Enemy/EnemyHealth.Health` (`CharacterAttributesComponent.health` (`self.attributes`)) _asenemy_health)
      (`Widget.SetVisibility` _asenemy_health "Visible")
      (if (< (/ Magnitude (`CharacterMovementComponent.Mass` _charactermovement)) 15.0)
        (`self.LaunchCharacter` (/ _returnvalue (/ (`CharacterMovementComponent.Mass` _charactermovement) 100.0)))
        (`CharacterMovementComponent.SetMovementMode` (`self.CharacterMovement`) "MOVE_Falling" 0)
        (else
          (`self.LaunchCharacter` (* _returnvalue (+ 250.0 0.0)))
          (`KismetSystemLibrary.Delay` 0.1))))))

(event `TakeFallDamage`
  ;[1 1 1] Fall Damage
  (set `self.FallDamageTimer` 0.0)
  (if (not (`self.Ragdolled`))
    (bind _returnvalue (`PrimitiveComponent.GetPhysicsLinearVelocity` (`self.CapsuleComponent`) "None"))
    (bind _returnvalue_2 (`KismetMathLibrary.VSize` _returnvalue))
    (if (> _returnvalue_2 (`self.FallDamageVelocityThreshold`))
      (bind _returnvalue_3 (* (- _returnvalue_2 (`self.FallDamageVelocityThreshold`)) (`self.FallDamageMultiplier`)))
      (`KismetSystemLibrary.PrintString` (`KismetStringLibrary.Conv_DoubleToString` _returnvalue_3))
      (`self.TakeDamage` _returnvalue_3 "HealthDamageType" null)
      (else
        (`KismetSystemLibrary.PrintString` "Fall damage threshold not met")))))

(event `self.OnHeal`
  (params (amount :type "Float (single-precision)") (healType :type "EDamageTypes Enum (by ref)" :default "HealthDamageType"))
  ;[1 1 1] On Heal
  (bind _asenemy_health (cast `/Game/BluePrints/UI/Enemy/EnemyHealth` (`WidgetComponent.GetWidget` (`self.HealthBar`))))
  (set `/Game/BluePrints/UI/Enemy/EnemyHealth.Health` (`CharacterAttributesComponent.health` (`self.attributes`)) _asenemy_health))

(event `ReceiveHitStop`
  (params (duration :type "Float (double-precision)"))
  ;[1 1 1] Hitstop
  (set `SkeletalMeshComponent.GlobalAnimRateScale` 0.0 (`self.Mesh`))
  (`KismetSystemLibrary.RetriggerableDelay` duration)
  (`CharacterMovementComponent.SetMovementMode` (`self.CharacterMovement`) "MOVE_Walking" 0)
  (set `SkeletalMeshComponent.GlobalAnimRateScale` 1.0 (`self.Mesh`)))

(event `self.ReceiveBeginPlay`
  ;[1 1 1] Set Enemy Health
  (bind _asenemy_health (cast `/Game/BluePrints/UI/Enemy/EnemyHealth` (`WidgetComponent.GetWidget` (`self.HealthBar`))))
  (set `/Game/BluePrints/UI/Enemy/EnemyHealth.MaxHealth` (`CharacterAttributesComponent.maxHealth` (`self.attributes`)) _asenemy_health)
  (set `/Game/BluePrints/UI/Enemy/EnemyHealth.Health` (`CharacterAttributesComponent.health` (`self.attributes`)) _asenemy_health)
  (`Widget.SetVisibility` _asenemy_health "Hidden")
  (set `self.FallDamageMultiplier` (/ (`CharacterMovementComponent.Mass` (`self.CharacterMovement`)) 100.0)))

(event `self.K2_OnMovementModeChanged`
  (params (PrevMovementMode :type "EMovementMode Enum" :default "MOVE_None") (NewMovementMode :type "EMovementMode Enum" :default "MOVE_None") (PrevCustomMode :type Byte) (NewCustomMode :type Byte))
  ;[1 1 1] Movement States
  (if (and (`|EnumEquality` PrevMovementMode "MOVE_Falling") (or (`|EnumEquality` NewMovementMode "MOVE_Walking") (`|EnumEquality` NewMovementMode "MOVE_NavWalking")))
    (if (`self.Ragdolled`)
      (if (> (`CharacterAttributesComponent.health` (`self.attributes`)) 0.0)
        (`KismetSystemLibrary.Delay` 3.0)
        (`self.EndRagdoll`))
      (else
        (`self.TakeFallDamage`)))))

(event `self.ReceiveHit`
  (params (MyComp :type "PrimitiveComponent Object Reference") (Other :type "Actor Object Reference") (OtherComp :type "PrimitiveComponent Object Reference") (bSelfMoved :type Boolean) (HitLocation :type "Vector Structure") (HitNormal :type "Vector Structure") (NormalImpulse :type "Vector Structure") (Hit :type "HitResult Structure (by ref)"))
  (bind (_bblockinghit _binitialoverlap _time _distance _location _impactpoint _normal _impactnormal) (`GameplayStatics.BreakHitResult` Hit))
  (bind _z (.z _impactnormal))
  ;[1 1 1] Hit Event
  (if (and (`self.Ragdolled`) (!= OtherComp (`self.Mesh`)) (> (`CharacterAttributesComponent.health` (`self.attributes`)) 0.0))
    (`self.RagdollCollideWithSurface` (`SceneComponent.GetComponentVelocity` (`self.Mesh`)) _impactnormal (0.0 0.0 -1.0) (`KismetMathLibrary.VSize` NormalImpulse))
    (if (and (>= _z (.x _impactnormal)) (>= _z (.y _impactnormal)) (> _z 0.0))
      (`self.EndRagdoll`))))

(event `self.OnTakeDamage`
  (params (amount :type "Float (single-precision)") (damageType :type "EDamageTypes Enum (by ref)" :default "HealthDamageType"))
  (bind _returnvalue (`self.GetController`))
  (bind _returnvalue_2 (`self.GetController`))
  (bind _capsulecomponent (`self.CapsuleComponent`))
  (bind (_returnvalue_roll _returnvalue_pitch _returnvalue_yaw) (`KismetMathLibrary.BreakRotator` (`SceneComponent.K2_GetComponentRotation` _capsulecomponent)))
  (bind _returnvalue_3 (`WidgetComponent.GetWidget` (`self.HealthBar`)))
  (bind (_returnvalue_roll_2 _returnvalue_pitch_2 _returnvalue_yaw_2) (`KismetMathLibrary.BreakRotator` (`KismetMathLibrary.FindLookAtRotation` (`SceneComponent.K2_GetComponentLocation` _capsulecomponent) (`SceneComponent.K2_GetComponentLocation` (`Character.Mesh` (`GameplayStatics.GetPlayerCharacter` 0))))))
  ;[1 1 1] Enemy Takes Damage
  ;;[1 1 1] Bloodsplat
  (`/Game/BluePrints/MythicismPlayer/C_Bloodsplat.SpawnBloodsplatter` (`self.C_Bloodsplat`) (* (`KismetMathLibrary.VSize` (`SceneComponent.K2_GetComponentScale` (`self.Mesh`))) 0.4) 1.0)
  ;;[1 1 1] Hit bar
  (bind _asenemy_health (cast `/Game/BluePrints/UI/Enemy/EnemyHealth` _returnvalue_3))
  (set `/Game/BluePrints/UI/Enemy/EnemyHealth.Health` (`CharacterAttributesComponent.health` (`self.attributes`)) _asenemy_health)
  (`Widget.SetVisibility` _returnvalue_3 "Visible")
  ;;[1 1 1] Get hit sound
  (`GameplayStatics.SpawnSoundAtLocation` (`self.getHitSound`) (`self.K2_GetActorLocation`) (struct) 1.0 1.0 0.0 null null)
  ;;[1 1 1] Turn to player
  (if (not (`self.Ragdolled`))
    (`/Engine/EditorBlueprintResources/StandardMacros.DoOnce` false
      (:`Completed`
        (bind (_direction _value) (`Timeline|Timeline_0` :!via `PlayFromStart`)
          (:`Update`
            (`SceneComponent.K2_SetWorldRotation` _capsulecomponent (`KismetMathLibrary.MakeRotator` _returnvalue_roll _returnvalue_pitch (`KismetMathLibrary.Lerp` _returnvalue_yaw _returnvalue_yaw_2 _value)) false false)
            (`KismetSystemLibrary.Delay` 0.7)
            ;[1 1 1] Activate behavior
            (if (`KismetSystemLibrary.IsValid` _returnvalue)
              (`BlackboardComponent.SetValueAsBool` (`AIBlueprintHelperLibrary.GetBlackboard` _returnvalue) "CanSeePlayer?" true)
              (`BlackboardComponent.SetValueAsBool` (`AIBlueprintHelperLibrary.GetBlackboard` _returnvalue_2) "TauntedPlayer" true :!label _label)
              (`SceneComponent.SetVisibility` (`self.weaponHand`) true false)
              (elif (`KismetSystemLibrary.IsValid` _returnvalue_2)
                (goto _label)))))))))

(event `self.OnDie`
  (bind _mesh (`self.Mesh`))
  (bind _cameratarget (`self.CameraTarget`))
  ;[1 1 1] Enemy Death
  (set `CharacterAttributesComponent.isInvincible` true (`self.attributes`))
  ;;[1 1 1] Bloodsplat
  (`/Game/BluePrints/MythicismPlayer/C_Bloodsplat.SpawnBloodsplatter` (`self.C_Bloodsplat`) (* (`KismetMathLibrary.VSize` (`SceneComponent.K2_GetComponentScale` (`self.Mesh`))) 0.4) 1.0)
  (if (`KismetSystemLibrary.IsValid` _cameratarget)
    (`ActorComponent.K2_DestroyComponent` _cameratarget))
  (bind _asenemy_health (cast `/Game/BluePrints/UI/Enemy/EnemyHealth` (`WidgetComponent.GetWidget` (`self.HealthBar`))))
  (set `/Game/BluePrints/UI/Enemy/EnemyHealth.Health` (`CharacterAttributesComponent.health` (`self.attributes`)) _asenemy_health)
  (`/Engine/EditorBlueprintResources/StandardMacros.DoOnce` false
    (:`Completed`
      (set `self.bUseControllerRotationYaw` false)
      (`CharacterMovementComponent.DisableMovement` (`self.CharacterMovement`))
      (`PrimitiveComponent.SetCollisionEnabled` (`self.CapsuleComponent`) "NoCollision")
      (`PrimitiveComponent.SetCollisionResponseToChannel` (`self.Mesh`) "ECC_PhysicsBody" "ECR_Ignore")
      (`GameplayStatics.SpawnSoundAtLocation` (`self.dieSound`) (`self.K2_GetActorLocation`) (struct) 1.0 1.0 0.0 null null)
      (`BrainComponent.StopLogic` (`AIController.BrainComponent` (`AIBlueprintHelperLibrary.GetAIController` self)) "dead")
      (`self.DetachFromControllerPendingDestroy`)
      (if (not (`self.Ragdolled`))
        (if (> (`KismetMathLibrary.RandomInteger` 2) 0)
          (`SkeletalMeshComponent.PlayAnimation` _mesh "/Game/Animations/ProSwordAndShield/swordandshielddeath_2_4UE4.swordandshielddeath_2_4UE4" false)
          (else
            (`SkeletalMeshComponent.PlayAnimation` _mesh "/Game/Animations/ProSwordAndShield/swordandshielddeath4UE4.swordandshielddeath4UE4" false)))
        (`KismetSystemLibrary.Delay` 2.0)
        (`PrimitiveComponent.SetSimulatePhysics` _mesh false))
      (bind _asthird_person_game_mode (cast `/Game/BluePrints/ThirdPersonCharacter/ThirdPersonGameMode` (`GameplayStatics.GetGameMode`)))
      (set `/Game/BluePrints/ThirdPersonCharacter/ThirdPersonGameMode.NumberOfEnemies` (- (`/Game/BluePrints/ThirdPersonCharacter/ThirdPersonGameMode.NumberOfEnemies` _asthird_person_game_mode) 1) _asthird_person_game_mode)
      (bind _returnvalue (`|SpawnActorFromClass` "/Game/BluePrints/SpellsAndCurses/EnemySpells/BP_FavorSpell.BP_FavorSpell_C" (`KismetMathLibrary.MakeTransform` (`self.K2_GetActorLocation` self)) "AlwaysSpawn" "OverrideRootScale" null null))
      (bind _asbp_mythicism_player (cast `/Game/BluePrints/MythicismPlayer/BP_MythicismPlayer` (`GameplayStatics.GetPlayerCharacter` 0)))
      (`/Game/BluePrints/SpellsAndCurses/EnemySpells/BP_FavorSpell.SetFavorAmount` _returnvalue (* (`/Game/BluePrints/MythicismPlayer/C_PlayerStats.FavorMultiplier` (`/Game/BluePrints/MythicismPlayer/BP_MythicismPlayer.C_PlayerStats` _asbp_mythicism_player)) (`self.favorAmount`)))
      (`KismetSystemLibrary.Delay` 3.0)
      (`self.K2_DestroyActor`))))

(fn `UserConstructionScript`)