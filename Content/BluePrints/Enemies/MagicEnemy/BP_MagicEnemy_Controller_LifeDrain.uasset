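; AI controller for the life-drain magic enemy, running its behavior tree on BeginPlay.
; AI perception updates for actors whose first tag is Player write the CanSeePlayer? flag and the playerCharacter reference to the blackboard.
; The first such update also sets focus on player pawn 0 through a DoOnce that is never reset.
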(event `self.ReceiveBeginPlay`
  ;[1 1 1] Run Behavior Tree
  (`self.RunBehaviorTree` "/Game/BluePrints/Enemies/MagicEnemy/MagicEnemy_LifeDrain_Tree.MagicEnemy_LifeDrain_Tree"))

(event `self.AIPerception.OnTargetPerceptionUpdated`
  (params (Actor :type "Actor Object Reference") (Stimulus :type "AIStimulus Structure"))
  ;[1 1 1] Sense Player
  (if (== (`|GetArrayItem` (`Actor.Tags` Actor)) "Player")
    (`BlackboardComponent.SetValueAsBool` (`AIBlueprintHelperLibrary.GetBlackboard` null) "CanSeePlayer?" (`.bSuccessfullySensed` (break `AIStimulus` Stimulus)))
    (`BlackboardComponent.SetValueAsObject` (`AIBlueprintHelperLibrary.GetBlackboard` null) "playerCharacter" Actor)
    (`/Engine/EditorBlueprintResources/StandardMacros.DoOnce` false
      (:`Completed`
        (`self.K2_SetFocus` (`GameplayStatics.GetPlayerPawn` 0))))))

(fn `UserConstructionScript`)