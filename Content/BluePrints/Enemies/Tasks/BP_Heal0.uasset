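; Behavior tree task in which the BP_arcangelEnemy boss heals itself.
; It spawns a heal particle effect below the pawn, sets the boss invincible and plays the Boss_Heal montage.
; On completion it restores a tenth of max health, clears the HealKey blackboard flag and updates the health bar widget.
; After a short delay it destroys the effect and finishes, setting invincibility to true again rather than clearing it.
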(event `self.ReceiveExecuteAI`
  (params (OwnerController :type "AIController Object Reference") (ControlledPawn :type "Pawn Object Reference"))
  (bind (_returnvalue_x _returnvalue_y _returnvalue_z) (`KismetMathLibrary.BreakVector` (`Actor.K2_GetActorLocation` ControlledPawn)))
  (bind _returnvalue (`GameplayStatics.SpawnEmitterAtLocation` "/Game/Particles/FXVarietyPack/P_BossHeal.P_BossHeal" (`KismetMathLibrary.MakeVector` _returnvalue_x _returnvalue_y (- _returnvalue_z 80.0))))
  (bind _asbp_arcangel_enemy (cast `/Game/BluePrints/Enemies/ArchAngelBoss/BP_arcangelEnemy` ControlledPawn)
    (:`then`
      (bind _attributes (`MythicismCharacter.attributes` _asbp_arcangel_enemy))
      (set `CharacterAttributesComponent.isInvincible` true _attributes)
      (`|PlayMontage` (`Character.Mesh` _asbp_arcangel_enemy) "/Game/Animations/Retargeted_Serath_Animations/Boss_Heal.Boss_Heal"
        (:`OnCompleted`
          (`MythicismCharacter.Heal` _asbp_arcangel_enemy (* (`CharacterAttributesComponent.maxHealth` _attributes) 0.1) "HealthDamageType")
          (`BTFunctionLibrary.SetBlackboardValueAsBool` (`self.HealKey`))
          (bind _returnvalue_2 (`WidgetComponent.GetWidget` (`/Game/BluePrints/Enemies/BP_Enemy_1_Character.HealthBar` _asbp_arcangel_enemy)))
          (bind _asenemy_health (cast `/Game/BluePrints/UI/Enemy/EnemyHealth` _returnvalue_2))
          (set `/Game/BluePrints/UI/Enemy/EnemyHealth.Health` (`CharacterAttributesComponent.health` (`MythicismCharacter.attributes` _asbp_arcangel_enemy)) _asenemy_health)
          (`Widget.SetVisibility` _returnvalue_2 "Visible")
          (`KismetSystemLibrary.Delay` 0.5)
          (`ActorComponent.K2_DestroyComponent` _returnvalue)
          (set `CharacterAttributesComponent.isInvincible` true _attributes)
          (`self.FinishExecute` true))))
    (:`CastFailed`
      (`self.FinishExecute` false))))