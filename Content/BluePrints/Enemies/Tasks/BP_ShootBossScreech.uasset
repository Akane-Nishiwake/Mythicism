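; Behavior tree task for the boss's screech attack, firing a projectile spell at the player.
; After a short wind-up it plays a slowed montage on the Enemy's mesh, then waits before spawning BP_Boss_Screech from the current weapon's location and the pawn's aim rotation.
; The short-lived screech is fired along the normalized direction from weapon to player, then the task finishes successfully.
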(event `self.ReceiveExecuteAI`
  (params (OwnerController :type "AIController Object Reference") (ControlledPawn :type "Pawn Object Reference"))
  (bind _asenemy (cast `Enemy` ControlledPawn :!pure true))
  (bind _returnvalue (`Actor.K2_GetActorLocation` (`MythicismCharacter.GetCurrentWeapon` _asenemy)))
  ;[1 1 1] Screech Boss attack
  (`KismetSystemLibrary.Delay` 0.75)
  (`|PlayMontage` (`Character.Mesh` _asenemy) "/Game/Animations/BorrowedAnimations/Burden_slow_Montage.Burden_slow_Montage" 0.3
    (:`then`
      (`KismetSystemLibrary.Delay` 1.2)
      (bind _returnvalue_2 (`|SpawnActorFromClass` "/Game/BluePrints/SpellsAndCurses/EnemySpells/BP_Boss_Screech.BP_Boss_Screech_C" (`KismetMathLibrary.ComposeTransforms` (`KismetMathLibrary.Conv_RotatorToTransform` (`Pawn.GetBaseAimRotation` ControlledPawn)) (`KismetMathLibrary.Conv_VectorToTransform` _returnvalue)) "AlwaysSpawn" "OverrideRootScale" null ControlledPawn))
      (`Actor.SetLifeSpan` _returnvalue_2 5.0)
      (`QuickSpell.FireSpell` _returnvalue_2 (`KismetMathLibrary.Normal` (- (`Actor.K2_GetActorLocation` (`GameplayStatics.GetPlayerCharacter` 0)) _returnvalue)))
      (`self.FinishExecute` true))))