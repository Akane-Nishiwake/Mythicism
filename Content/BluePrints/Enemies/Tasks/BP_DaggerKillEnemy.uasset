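; Behavior tree task that has an Enemy play a one-time dagger-sheathe flourish with a boast, commented as a reaction to first seeing the player.
; A DoOnce gate leads through delays to the montage, a random choice of two voice lines and a movement stop.
; The weapon hand is then hidden, also on montage interruption, and the task finishes as failed.
; Later executions of the same instance stop at the gate without finishing.
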(event `self.ReceiveExecuteAI`
  (params (OwnerController :type "AIController Object Reference") (ControlledPawn :type "Pawn Object Reference"))
  (bind _asenemy (cast `Enemy` ControlledPawn :!pure true))
  (bind _returnvalue (`Actor.K2_GetActorLocation` _asenemy))
  ;[1 1 1] Play single animation first time seeing player
  (`/Engine/EditorBlueprintResources/StandardMacros.DoOnce` false
    (:`Completed`
      (`KismetSystemLibrary.Delay` 1.0)
      (`|PlayMontage` (`Character.Mesh` _asenemy) "/Game/Animations/ProSwordAndShield/Dagger_Sheathe.Dagger_Sheathe" 0.8
        (:`then`
          (if (> (`KismetMathLibrary.RandomInteger` 2) 0)
            (`GameplayStatics.PlaySoundAtLocation` "/Game/Audio/VoicesPack/Gideon_Intro_Boast_030.Gideon_Intro_Boast_030" _returnvalue (struct) 0.85 1.3 0.0 null null null)
            (else
              (`GameplayStatics.PlaySoundAtLocation` "/Game/Audio/VoicesPack/Revenant_Intro_Boast_010.Revenant_Intro_Boast_010" _returnvalue (struct) 0.85 1.0 0.0 null null null)))
          (`Controller.StopMovement` OwnerController)
          (`KismetSystemLibrary.Delay` 0.8))
        (:`OnInterrupted`
          _))
      (`SceneComponent.SetVisibility` (`MythicismCharacter.weaponHand` _asenemy) false false)
      (`KismetSystemLibrary.Delay` 1.0)
      (`Controller.StopMovement` OwnerController)
      (`self.FinishExecute` false))))