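; Behavior tree task where the archangel boss calls a telegraphed lightning strike on the player.
; It captures the player's location at the start, plays the boss's lightning montage and spawns a growing warning light at that spot.
; After a delay it drops a lightning actor there with a camera shake, then plays thunder and finishes successfully.
; Because the target is never updated, the player can move away during the warning.
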(event `self.ReceiveExecuteAI`
  (params (OwnerController :type "AIController Object Reference") (ControlledPawn :type "Pawn Object Reference"))
  ;[1 1 1] Boss Lightning Strike
  (bind _asbp_arcangel_enemy (cast `/Game/BluePrints/Enemies/ArchAngelBoss/BP_arcangelEnemy` ControlledPawn))
  (bind _output_get (set `self.StrikeLocation` (`Actor.K2_GetActorLocation` (`GameplayStatics.GetPlayerCharacter` 0))))
  (`Character.PlayAnimMontage` _asbp_arcangel_enemy "/Game/BluePrints/Enemies/ArchAngelBoss/AngelAnims/Lighting/Angel_Lightning.Angel_Lightning" 0.5 "None")
  (bind _returnvalue (`|SpawnActorFromClass` "/Game/BluePrints/Enemies/ArchAngelBoss/ExtraBP/BP_PointLight.BP_PointLight_C" (`KismetMathLibrary.MakeTransform` _output_get) "Undefined" "OverrideRootScale" null null))
  (`/Game/BluePrints/Enemies/ArchAngelBoss/ExtraBP/BP_PointLight.WarningGrow` _returnvalue)
  (`KismetSystemLibrary.Delay` 1.5)
  (bind _returnvalue_2 (`|SpawnActorFromClass` "/Game/BluePrints/Enemies/ArchAngelBoss/ExtraBP/BP_Lightning.BP_Lightning_C" (`KismetMathLibrary.MakeTransform` _output_get) "Undefined" "OverrideRootScale" null null))
  (`GameplayStatics.PlayWorldCameraShake` "/Game/BluePrints/UI/BP_Boss_LightningShake.BP_Boss_LightningShake_C" _output_get 0.0 2000.0 1.0 true)
  (`/Game/BluePrints/Enemies/ArchAngelBoss/ExtraBP/BP_Lightning.LightningDrop` _returnvalue_2)
  (`KismetSystemLibrary.Delay` 0.2)
  (`GameplayStatics.SpawnSoundAtLocation` "/Game/Audio/BossSounds/Thunder_Boss_Noise_Cue.Thunder_Boss_Noise_Cue" _output_get (struct) 1.0 1.0 0.0 null null)
  (`self.FinishExecute` true))