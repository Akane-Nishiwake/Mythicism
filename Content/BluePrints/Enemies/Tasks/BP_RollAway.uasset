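; Behavior tree task that makes an enemy roll sideways, succeeding only if a clear destination is found.
; Line-traces a random side, retrying if blocked with a separately randomized direction that can repeat the same side.
; Clears focus and raises walk speed, then runs AIMoveTo and the roll montage in parallel.
; Once both end, or no spot is found, it focuses on the player, restores speed and finishes.
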(event `self.ReceiveExecuteAI`
  (params (OwnerController :type "AIController Object Reference") (ControlledPawn :type "Pawn Object Reference"))
  ;[1 1 1] Start task
  (`AIController.K2_SetFocus` OwnerController null)
  (bind _output_get (set `self.Enemy` (cast `Enemy` ControlledPawn :!pure true)))
  (bind _charactermovement (`Character.CharacterMovement` _output_get))
  (set `self.previousWalkSpeed` (`MovementComponent.GetMaxSpeed` _charactermovement))
  (set `CharacterMovementComponent.MaxWalkSpeed` 720.0 _charactermovement)
  ;[1 1 1] Move Enemy to Location
  (bind (_safedestinationfound_ _rolldestination) (`self.DetermineRollDest`))
  (if _safedestinationfound_
    (`|AIMoveTo` (`self.Enemy`) _rolldestination null 5.0 true
      (:`then`
        ;[1 1 1] Roll animation
        (`|PlayMontage` (`Character.Mesh` (`self.Enemy`)) "/Game/Animations/Mannequin/Moving_EnemyRoll_Montage.Moving_EnemyRoll_Montage"
          (:`then`)
          (:`OnCompleted`
            (set `self.finishedAnimating` true)
            (`self.TryFinsihTask`))))
      (:`OnSuccess`
        (set `self.finishedMoving` true :!label _label)
        (`self.TryFinsihTask`))
      (:`OnFail`
        (goto _label)))
    (else
      (set `self.finishedAnimating` true)
      (goto _label))))

(event `TryFinsihTask`
  ;[1 1 1] Finish task
  (if (and (`self.finishedAnimating`) (`self.finishedMoving`))
    (`AIController.K2_SetFocus` (stale `self.ReceiveExecuteAI` OwnerController) (`GameplayStatics.GetPlayerPawn` 0))
    (set `CharacterMovementComponent.MaxWalkSpeed` (`self.previousWalkSpeed`) (`Character.CharacterMovement` (`self.Enemy`)))
    (`self.FinishExecute` (`self.raycastResult`))))

(fn `DetermineRollDest`
  (returns (`SafeDestinationFound?` :type Boolean) (RollDestination :type "Vector Structure"))
  (locals (destination :type "Vector Structure") (direction :type "Float (double-precision)"))
  (bind _enemy (`self.Enemy`))
  (bind _enemy_2 (`self.Enemy`))
  (bind _returnvalue (`Actor.K2_GetActorLocation` _enemy))
  (bind _returnvalue_2 (`KismetMathLibrary.Conv_IntToDouble` (`self.RandomPlusOrMinus`)))
  (bind _returnvalue_3 (`Actor.K2_GetActorLocation` _enemy_2))
  ;[1 1 1] Raycast random direction
  (set `local.direction` _returnvalue_2)
  (bind _output_get (set `local.destination` (+ _returnvalue_3 (* (* (`Actor.GetActorRightVector` _enemy_2) _returnvalue_2) (`self.rollDistance`)))))
  (bind (_outhit _returnvalue_4) (`KismetSystemLibrary.LineTraceSingle` _returnvalue_3 _output_get "TraceTypeQuery1"))
  (set `self.raycastResult` (not _returnvalue_4))
  (if _returnvalue_4
    ;[1 1 1] Cast the other direction
    (bind _output_get_2 (set `local.destination` (+ _returnvalue (* (* (`Actor.GetActorRightVector` _enemy) (* (`local.direction`) -1.0)) (`self.rollDistance`)))))
    (bind (_outhit_2 _returnvalue_5) (`KismetSystemLibrary.LineTraceSingle` _returnvalue _output_get_2 "TraceTypeQuery1"))
    (set `self.raycastResult` (not _returnvalue_5)))
  ;[1 1 1] Return results
  (return (`self.raycastResult`) (`local.destination`)))

(fn `RandomPlusOrMinus`
  (returns (return :type Integer))
  (return (- (* (`KismetMathLibrary.RandomInteger` 2) 2) 1)))