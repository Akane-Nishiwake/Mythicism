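; Behavior tree task that picks a backup location directly behind an enemy.
; It sets the enemy's walk speed to BackupSpeed and writes a point a fixed distance behind the mesh, along the pawn's reversed forward vector, to a Blackboard key.
; The point is not validated against navigation or obstacles.
; It draws a debug line to the point and finishes successfully after a short delay.
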(event `self.ReceiveExecuteAI`
  (params (OwnerController :type "AIController Object Reference") (ControlledPawn :type "Pawn Object Reference"))
  (bind _asenemy (cast `Enemy` ControlledPawn :!pure true))
  (bind _returnvalue (`SceneComponent.K2_GetComponentLocation` (`Character.Mesh` _asenemy)))
  (bind _returnvalue_2 (+ _returnvalue (* (`Actor.GetActorForwardVector` ControlledPawn) -400.0)))
  ;[1 1 1] Set Strafe Location
  (set `CharacterMovementComponent.MaxWalkSpeed` (`self.BackupSpeed`) (`Character.CharacterMovement` _asenemy))
  (`KismetSystemLibrary.DrawDebugLine` _returnvalue _returnvalue_2 (struct :`R` 0.90625 :`G` 0.245375 :`B` 0.747406 :`A` 1.0) 10.0 5.0)
  (`BTFunctionLibrary.SetBlackboardValueAsVector` (`self.BBRef`) _returnvalue_2)
  (`KismetSystemLibrary.Delay` 0.1)
  (`self.FinishExecute` true))