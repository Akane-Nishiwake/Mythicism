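; Behavior tree task that makes an Enemy back away from its current position, presumably for magic users.
; On execute it caches the walk speed, applies BackupSpeed and runs AI MoveTo to a point BackupDistance behind its forward vector.
; Whether the move succeeds or fails, it restores the cached speed and finishes the task as successful.
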(event `self.ReceiveExecuteAI`
  (params (OwnerController :type "AIController Object Reference") (ControlledPawn :type "Pawn Object Reference"))
  (bind _asenemy (cast `Enemy` ControlledPawn :!pure true))
  (bind _charactermovement (`Character.CharacterMovement` _asenemy))
  ;[1 1 1] Start task
  (set `self.defaultspeed` (`CharacterMovementComponent.MaxWalkSpeed` _charactermovement))
  ;[1 1 1] Set backup speed
  (set `CharacterMovementComponent.MaxWalkSpeed` (`self.BackupSpeed`) _charactermovement)
  ;[1 1 1] Backup
  (`|AIMoveTo` ControlledPawn (+ (`Actor.K2_GetActorLocation` _asenemy) (* (`Actor.GetActorForwardVector` _asenemy) (* (`self.BackupDistance`) -1.0))) null 5.0 true
    (:`OnSuccess`
      _)
    (:`OnFail`
      _))
  ;[1 1 1] Finish task
  (set `CharacterMovementComponent.MaxWalkSpeed` (`self.defaultspeed`) (`Character.CharacterMovement` _asenemy))
  (`self.FinishExecute` true))