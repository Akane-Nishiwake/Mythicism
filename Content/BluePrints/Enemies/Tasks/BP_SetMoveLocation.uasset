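; Behavior tree task for the enemy AI that writes the player reference and location to the blackboard as a pursuit target, then finishes.
; A separate Reset event holds attack logic: a montage, then a random choice between re-entering the DoOnce and strafing to a debug-drawn forward-right offset.
; Execute never calls that event, and the pursuit speed change is disconnected.
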(event `Reset`
  ;[1 1 1] Attack Player
  (`/Engine/EditorBlueprintResources/StandardMacros.DoOnce` false :!via `Reset` :!label _label
    (:`Completed`
      (bind _asbp_enemy_1_character (cast `/Game/BluePrints/Enemies/BP_Enemy_1_Character` (stale `self.ReceiveExecuteAI` ControlledPawn) :!pure true))
      (bind _mesh (`Character.Mesh` _asbp_enemy_1_character))
      (`|PlayMontage` _mesh null 0.8
        (:`OnCompleted`
          (`self.Reset`)
          (`KismetSystemLibrary.Delay` 0.2)
          (if (< (`KismetMathLibrary.RandomInteger` 3) 2)
            ;[1 1 1] Strafe Player
            (set `CharacterMovementComponent.MaxWalkSpeed` (`self.strafeSpeed`) (`Character.CharacterMovement` _asbp_enemy_1_character))
            (bind _returnvalue (`SceneComponent.K2_GetComponentLocation` _mesh))
            (bind _returnvalue_2 (+ _returnvalue (* (`Actor.GetActorForwardVector` (stale `self.ReceiveExecuteAI` ControlledPawn)) 50.0) (* (`Actor.GetActorRightVector` (stale `self.ReceiveExecuteAI` ControlledPawn)) 150.0)))
            (`KismetSystemLibrary.DrawDebugLine` _returnvalue _returnvalue_2 (struct :`R` 0.90625 :`G` 0.245375 :`B` 0.747406 :`A` 1.0) 10.0 5.0)
            (`BTFunctionLibrary.SetBlackboardValueAsVector` (`self.blackboardRef`) _returnvalue_2)
            (`KismetSystemLibrary.Delay` 2.0)
            (`self.FinishExecute` true)
            (else
              (goto _label))))))))

(event `self.ReceiveExecuteAI`
  (params (OwnerController :type "AIController Object Reference") (ControlledPawn :type "Pawn Object Reference"))
  (bind _outactors (`GameplayStatics.GetAllActorsOfClass` "/Game/BluePrints/MythicismPlayer/BP_MythicismPlayer.BP_MythicismPlayer_C"))
  (bind _output (`|GetArrayItem` _outactors))
  (`BTFunctionLibrary.SetBlackboardValueAsObject` (`self.blackboardPlayerRef`) _output)
  ;[1 1 1] Pursue Player
  (`BTFunctionLibrary.SetBlackboardValueAsVector` (`self.blackboardRef`) (`Actor.K2_GetActorLocation` _output))
  (`self.FinishExecute` true))