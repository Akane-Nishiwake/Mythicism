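; Behavior tree task for the boss that moves to the blackboard strafe location, then attacks.
; It clears focus, flags IsAttacking and plays a random Attack1 or Attack3 weapon montage, restoring player focus afterward.
; Attack3 also starts a delayed lightning strike for the archangel enemy: a warning light at the player's sampled position, then a bolt, camera shake and thunder.
; An Attack2 branch is present but disconnected.
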(event `self.ReceiveExecuteAI`
  (params (OwnerController :type "AIController Object Reference") (ControlledPawn :type "Pawn Object Reference"))
  (bind _asenemy (cast `Enemy` ControlledPawn :!pure true))
  (bind _returnvalue (`MythicismCharacter.GetCurrentWeapon` _asenemy))
  (bind _mesh (`Character.Mesh` _asenemy))
  (bind _attack1 (`Weapon.attack1` _returnvalue))
  ;[1 1 1] Move Enemy to Location
  (`|AIMoveTo` ControlledPawn (`BTFunctionLibrary.GetBlackboardValueAsVector` (`self.BBRef_StrafeLocation`)) null
    (:`then`
      (`Controller.StopMovement` OwnerController)
      (`AIController.K2_ClearFocus` OwnerController)
      ;[1 1 1] Get Enemy Current Weapon
      (`/Engine/EditorBlueprintResources/StandardMacros.DoOnce` false :!label _label
        (:`Completed`
          (`BTFunctionLibrary.SetBlackboardValueAsBool` (`self.BBRef_IsAttacking`) true)
          ;[1 1 1] Attack and Dodge Animation
          (if (< (`KismetMathLibrary.RandomInteger` 4) 1)
            (`|PlayMontage` _mesh _attack1
              (:`OnCompleted`
                _)
              (:`OnInterrupted`
                _))
            (`KismetSystemLibrary.Delay` 0.2 :!label _label_2)
            (`self.Reset`)
            (`BTFunctionLibrary.SetBlackboardValueAsBool` (`self.BBRef_IsAttacking`))
            (`AIController.K2_SetFocus` OwnerController (`GameplayStatics.GetPlayerCharacter` 0))
            (`self.FinishExecute` true)
            (else
              (switch `int` (`KismetMathLibrary.RandomInteger` 3)
                (:`0`
                  (`|PlayMontage` _mesh _attack1
                    (:`OnCompleted`
                      (goto _label_2))
                    (:`OnInterrupted`
                      (goto _label_2))))
                (:`1`
                  _)
                (:`2`
                  _))
              (`|PlayMontage` _mesh (`Weapon.attack3` _returnvalue)
                (:`then`
                  ;[1 0.9519 0.1275] Lightning strike continuation
                  (`KismetSystemLibrary.Delay` 4.0)
                  (cast `/Game/BluePrints/Enemies/ArchAngelBoss/BP_arcangelEnemy` ControlledPawn)
                  (bind _output_get (set `self.Strike Location` (`Actor.K2_GetActorLocation` (`GameplayStatics.GetPlayerCharacter` 0))))
                  (bind _returnvalue_2 (`|SpawnActorFromClass` "/Game/BluePrints/Enemies/ArchAngelBoss/ExtraBP/BP_PointLight.BP_PointLight_C" (`KismetMathLibrary.MakeTransform` _output_get) "Undefined" "OverrideRootScale" null null))
                  (`/Game/BluePrints/Enemies/ArchAngelBoss/ExtraBP/BP_PointLight.WarningGrow` _returnvalue_2)
                  (`KismetSystemLibrary.Delay` 1.5)
                  (bind _returnvalue_3 (`|SpawnActorFromClass` "/Game/BluePrints/Enemies/ArchAngelBoss/ExtraBP/BP_Lightning.BP_Lightning_C" (`KismetMathLibrary.MakeTransform` _output_get) "Undefined" "OverrideRootScale" null null))
                  (`GameplayStatics.PlayWorldCameraShake` "/Game/BluePrints/UI/BP_Boss_LightningShake.BP_Boss_LightningShake_C" _output_get 0.0 2000.0 1.0 true)
                  (`/Game/BluePrints/Enemies/ArchAngelBoss/ExtraBP/BP_Lightning.LightningDrop` _returnvalue_3)
                  (`KismetSystemLibrary.Delay` 0.2)
                  (`GameplayStatics.SpawnSoundAtLocation` "/Game/Audio/BossSounds/Thunder_Boss_Noise_Cue.Thunder_Boss_Noise_Cue" _output_get (struct) 1.0 1.0 0.0 null null)
                  (`self.FinishExecute` true))
                (:`OnCompleted`
                  (goto _label_2))
                (:`OnInterrupted`
                  (goto _label_2))))))))))

(event `Reset`
  ;[1 1 1] Get Enemy Current Weapon
  (goto _label :!via `Reset`))