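; Behavior tree task that runs an enemy's charge attack.
; It stops AI movement, sets the charging Blackboard flag, clears focus and plays one of three random attack montages from the current weapon.
; The second attack also fires delayed slam particles on heavy or light hammers.
; Any montage completion, blend-out or interruption leads to an in-place recovery montage, whose completion or blend-out finishes the task successfully.
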(event `self.ReceiveExecuteAI`
  (params (OwnerController :type "AIController Object Reference") (ControlledPawn :type "Pawn Object Reference"))
  (bind _asenemy (cast `Enemy` ControlledPawn :!pure true))
  (bind _returnvalue (`MythicismCharacter.GetCurrentWeapon` _asenemy))
  (bind _mesh (`Character.Mesh` _asenemy))
  ;[1 1 1] Charge attack
  (`Controller.StopMovement` OwnerController)
  (`BTFunctionLibrary.SetBlackboardValueAsBool` (`self.BBRef_IsCharging`) true)
  (`AIController.K2_ClearFocus` OwnerController)
  (switch `int` (`KismetMathLibrary.RandomInteger` 3)
    (:`0`
      (`|PlayMontage` _mesh (`Weapon.attack1` _returnvalue) 1.5
        (:`OnCompleted`
          _)
        (:`OnBlendOut`
          _)
        (:`OnInterrupted`
          _))
      (`|PlayMontage` _mesh "/Game/Animations/BorrowedAnimations/InPlace_ChargerRecover_Montage.InPlace_ChargerRecover_Montage" 1.5 :!label _label
        (:`OnCompleted`
          _)
        (:`OnBlendOut`
          _))
      (`self.FinishExecute` true))
    (:`1`
      (`|PlayMontage` _mesh (`Weapon.attack2` _returnvalue) 1.4
        (:`then`
          (`KismetSystemLibrary.Delay` 1.5)
          (bind _asbp_enemy_hammer_heavy (cast `/Game/BluePrints/Weapons/Enemies/BP_EnemyHammer_Heavy` _returnvalue)
            (:`then`
              (`ActorComponent.Activate` (`/Game/BluePrints/Weapons/Enemies/BP_EnemyHammer_Heavy.SlamParticles` _asbp_enemy_hammer_heavy) true))
            (:`CastFailed`
              (bind _asbp_enemy_hammer_light (cast `/Game/BluePrints/Weapons/Enemies/BP_EnemyHammer_Light` _returnvalue))
              (`ActorComponent.Activate` (`/Game/BluePrints/Weapons/Enemies/BP_EnemyHammer_Light.SlamParticles` _asbp_enemy_hammer_light) true))))
        (:`OnCompleted`
          (goto _label))
        (:`OnBlendOut`
          (goto _label))
        (:`OnInterrupted`
          (goto _label))))
    (:`2`
      (`|PlayMontage` _mesh (`Weapon.attack3` _returnvalue) 1.4
        (:`OnCompleted`
          (goto _label))
        (:`OnBlendOut`
          (goto _label))
        (:`OnInterrupted`
          (goto _label))))))