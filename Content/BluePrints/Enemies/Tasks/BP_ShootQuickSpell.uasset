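; Behavior tree task that makes an enemy cast a quick spell at the player.
; It plays a moving cast montage, spawns the spell at the weapon after a short delay, and finishes when the montage completes.
; A forward line trace sets horizontal fire direction, while vertical aim comes from the direction to the player's capsule.
; The StopMovement call is disconnected, so the task does not halt the enemy.
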(event `self.ReceiveExecuteAI`
  (params (OwnerController :type "AIController Object Reference") (ControlledPawn :type "Pawn Object Reference"))
  (bind (_asenemy _bsuccess) (cast `Enemy` ControlledPawn :!pure true))
  (bind _caster (`self.Caster`))
  (bind (_firedirection_x _firedirection_y) (`KismetMathLibrary.BreakVector` (`self.FireDirection`)))
  (bind _caster_2 (`self.Caster`))
  (bind _caster_3 (`self.Caster`))
  (bind _returnvalue (`Actor.GetActorForwardVector` _caster))
  (bind _returnvalue_2 (`Actor.K2_GetActorLocation` (`self.Spell`)))
  (bind (_returnvalue_x _returnvalue_y _returnvalue_z) (`KismetMathLibrary.BreakVector` (- (`SceneComponent.K2_GetComponentLocation` (`Character.CapsuleComponent` (`GameplayStatics.GetPlayerCharacter` 0))) (`SceneComponent.K2_GetComponentLocation` (`QuickSpell.hitCollider` (`self.Spell`))))))
  (bind _returnvalue_3 (+ (* _returnvalue 100.0) (`Actor.K2_GetActorLocation` _caster)))
  (bind (_returnvalue_x_2 _returnvalue_y_2 _returnvalue_z_2) (`KismetMathLibrary.BreakVector` (`KismetMathLibrary.Normal` (`KismetMathLibrary.MakeVector` _returnvalue_x _returnvalue_y _returnvalue_z))))
  ;[1 1 1] Get caster
  (set `self.Caster` _asenemy)
  (if _bsuccess
    ;[1 1 1] Animate
    (`|PlayMontage` (`Character.Mesh` (`self.Caster`)) "/Game/Animations/Mannequin/Moving_EnemyQuickSpell_Montage.Moving_EnemyQuickSpell_Montage" 0.8
      (:`then`
        (`KismetSystemLibrary.Delay` 0.5)
        ;[1 1 1] Spawn spell
        (bind _returnvalue_4 (`|SpawnActorFromClass` (`self.SpellType`) (`KismetMathLibrary.ComposeTransforms` (`KismetMathLibrary.Conv_RotatorToTransform` (`Pawn.GetBaseAimRotation` _caster_2)) (`KismetMathLibrary.Conv_VectorToTransform` (`Actor.K2_GetActorLocation` (`MythicismCharacter.GetCurrentWeapon` _caster_2)))) "AlwaysSpawn" "OverrideRootScale" null _caster_3))
        (bind _output_get (set `self.Spell` _returnvalue_4))
        (set `Spell.spellCaster` _caster_3 _output_get)
        ;[1 1 1] FireSpell
        (bind _output_get_2 (set `self.TargetPoint` (+ (* _returnvalue 9000.0) _returnvalue_3)))
        (bind _outhit (`KismetSystemLibrary.LineTraceSingle` _returnvalue_3 _output_get_2 "TraceTypeQuery1"))
        (if (`GameplayStatics.BreakHitResult` _outhit)
          (set `self.FireDirection` (`KismetMathLibrary.Normal` (- (`.ImpactPoint` (`GameplayStatics.BreakHitResult` _outhit)) _returnvalue_2)))
          (else
            (set `self.FireDirection` (`KismetMathLibrary.Normal` (- (`self.TargetPoint`) _returnvalue_2)))))
        (set `self.FireDirection` (`KismetMathLibrary.MakeVector` _firedirection_x _firedirection_y _returnvalue_z_2))
        (`QuickSpell.FireSpell` (`self.Spell`) (`self.FireDirection`)))
      (:`OnCompleted`
        (`self.FinishExecute` true)))))