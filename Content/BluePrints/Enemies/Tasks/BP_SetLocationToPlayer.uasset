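; Behavior tree task that points an AI enemy at the player for pursuit.
; It finds the first BP_MythicismPlayer in the world and writes that actor and its current location to blackboard keys.
; It also sets the controlled Enemy's max walk speed to PursuitSpeed, then finishes with success immediately.
; The location is a one-time snapshot taken each time the task executes.
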(event `self.ReceiveExecuteAI`
  (params (OwnerController :type "AIController Object Reference") (ControlledPawn :type "Pawn Object Reference"))
  ;[1 1 1] Set Location to Player Position
  (bind _outactors (`GameplayStatics.GetAllActorsOfClass` "/Game/BluePrints/MythicismPlayer/BP_MythicismPlayer.BP_MythicismPlayer_C"))
  (bind _output (`|GetArrayItem` _outactors))
  (`BTFunctionLibrary.SetBlackboardValueAsObject` (`self.BBRef_PlayerCharacter`) _output)
  (set `CharacterMovementComponent.MaxWalkSpeed` (`self.pursuitSpeed`) (`Character.CharacterMovement` (cast `Enemy` ControlledPawn :!pure true)))
  (`BTFunctionLibrary.SetBlackboardValueAsVector` (`self.BBRefVector`) (`Actor.K2_GetActorLocation` _output))
  (`self.FinishExecute` true))