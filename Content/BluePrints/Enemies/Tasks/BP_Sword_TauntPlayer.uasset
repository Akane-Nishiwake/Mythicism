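; Behavior tree task that makes a sword enemy taunt the first time it sees the player.
; It plays an over-shoulder equip montage with a taunt sound, stops movement, then reveals the hand weapon after a short delay.
; It sets the TauntedPlayer blackboard flag and finishes after another delay.
; Montage completion jumps straight to setting the flag, while interruption also reveals the weapon first.
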(event `self.ReceiveExecuteAI`
  (params (OwnerController :type "AIController Object Reference") (ControlledPawn :type "Pawn Object Reference"))
  (bind _asenemy (cast `Enemy` ControlledPawn :!pure true))
  ;[1 1 1] Play single animation first time seeing player
  (`|PlayMontage` (`Character.Mesh` _asenemy) "/Game/Animations/ProMeleeAxePack/Enemy_EquipOverSHoulder.Enemy_EquipOverSHoulder" 0.8
    (:`then`
      (`GameplayStatics.PlaySoundAtLocation` "/Game/Audio/EnemyTaunts/SkeletonEnemyTaunt.SkeletonEnemyTaunt" (`Actor.K2_GetActorLocation` _asenemy) (struct) 0.85 1.0 0.0 null null null)
      (`Controller.StopMovement` OwnerController)
      (`KismetSystemLibrary.Delay` 0.8)
      (`SceneComponent.SetVisibility` (`MythicismCharacter.weaponHand` _asenemy) true false :!label _label))
    (:`OnCompleted`
      _)
    (:`OnInterrupted`
      (goto _label)))
  (`BTFunctionLibrary.SetBlackboardValueAsBool` (`self.TauntedPlayer`) true)
  (`KismetSystemLibrary.Delay` 1.0)
  (`self.FinishExecute` true))