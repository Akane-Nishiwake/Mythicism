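; Behavior tree task that moves an enemy to the player actor from the blackboard and performs a melee-range attack.
; On arrival, a DoOnce gate sets the attacking blackboard flag and plays one of three random attack montages from the enemy's current weapon.
; When the montage completes or is interrupted, a short delay precedes reopening the gate, clearing the flag and finishing successfully; failed moves have no handler.
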(event `self.ReceiveExecuteAI`
  (params (OwnerController :type "AIController Object Reference") (ControlledPawn :type "Pawn Object Reference"))
  (bind _asenemy (cast `Enemy` ControlledPawn :!pure true))
  (bind _returnvalue (`MythicismCharacter.GetCurrentWeapon` _asenemy))
  (bind _mesh (`Character.Mesh` _asenemy))
  ;[1 1 1] Move enemy to Player Actor
  (`|AIMoveTo` null (0.0 0.0 0.0) (`BTFunctionLibrary.GetBlackboardValueAsActor` (`self.PlayerCharacter`)) 10.0
    (:`OnSuccess`
      ;[1 1 1] Get Enemy Current Weapon
      (`/Engine/EditorBlueprintResources/StandardMacros.DoOnce` false :!label _label
        (:`Completed`
          (`BTFunctionLibrary.SetBlackboardValueAsBool` (`self.BBRef_IsAttacking`) true)
          ;[1 1 1] Attack and Dodge Animation
          (switch `int` (`KismetMathLibrary.RandomInteger` 3)
            (:`0`
              (`|PlayMontage` _mesh (`Weapon.attack1` _returnvalue) 1.5 1.4
                (:`OnCompleted`
                  _)
                (:`OnInterrupted`
                  _)))
            (:`1`
              (`|PlayMontage` _mesh (`Weapon.attack2` _returnvalue) 1.4
                (:`OnCompleted`
                  _)
                (:`OnInterrupted`
                  _)))
            (:`2`
              (`|PlayMontage` _mesh (`Weapon.attack3` _returnvalue) 1.4
                (:`OnCompleted`
                  _)
                (:`OnInterrupted`
                  _))))
          (`KismetSystemLibrary.Delay` 0.2)
          (`self.Reset`)
          (`BTFunctionLibrary.SetBlackboardValueAsBool` (`self.BBRef_IsAttacking`))
          (`self.FinishExecute` true))))))

(event `Reset`
  ;[1 1 1] Get Enemy Current Weapon
  (goto _label :!via `Reset`))