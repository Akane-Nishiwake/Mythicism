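; Behavior Tree task that prepares an Enemy to back away.
; On execute it sets the pawn's max walk speed to the backup speed, then writes a point a fixed distance behind the enemy's mesh, along its reversed forward vector, to the strafe location Blackboard key.
; It finishes successfully at once and does not move the pawn itself.
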(event `self.ReceiveExecuteAI`
  (params (OwnerController :type "AIController Object Reference") (ControlledPawn :type "Pawn Object Reference"))
  (bind _asenemy (cast `Enemy` ControlledPawn :!pure true))
  ;[1 1 1] Set Strafe Location
  (set `CharacterMovementComponent.MaxWalkSpeed` (`self.BackupSpeed`) (`Character.CharacterMovement` _asenemy))
  (`BTFunctionLibrary.SetBlackboardValueAsVector` (`self.BBRef_StrafeLocation`) (+ (`SceneComponent.K2_GetComponentLocation` (`Character.Mesh` _asenemy)) (* (`Actor.GetActorForwardVector` ControlledPawn) -250.0)))
  (`self.FinishExecute` true))