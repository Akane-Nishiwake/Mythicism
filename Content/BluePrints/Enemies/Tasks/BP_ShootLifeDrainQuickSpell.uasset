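; Behavior Tree task that makes an enemy cast a quick life-drain spell at the player.
; After a short delay, a random roll usually selects the cast; otherwise the task waits briefly and finishes successfully without casting.
; A cast plays a montage, then after another delay spawns the spell at the current weapon's location, sets the caster and fires it toward the first player's position before finishing.
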(event `self.ReceiveExecuteAI`
  (params (OwnerController :type "AIController Object Reference") (ControlledPawn :type "Pawn Object Reference"))
  (bind _asenemy (cast `Enemy` ControlledPawn :!pure true))
  (bind _returnvalue (`Actor.K2_GetActorLocation` (`MythicismCharacter.GetCurrentWeapon` _asenemy)))
  (`KismetSystemLibrary.Delay` 0.75)
  (if (> (`KismetMathLibrary.RandomInteger` 11) 2)
    ;[1 1 1] Quick Spell
    (`|PlayMontage` (`Character.Mesh` _asenemy) "/Game/Animations/BorrowedAnimations/Burden_slow_Montage.Burden_slow_Montage"
      (:`then`
        (`KismetSystemLibrary.Delay` 0.5)
        (bind _returnvalue_2 (`|SpawnActorFromClass` "/Game/BluePrints/SpellsAndCurses/EnemySpells/BP_EnemyQuickSpell-LifeDrain.BP_EnemyQuickSpell-LifeDrain_C" (`KismetMathLibrary.ComposeTransforms` (`KismetMathLibrary.Conv_RotatorToTransform` (`Pawn.GetBaseAimRotation` ControlledPawn)) (`KismetMathLibrary.Conv_VectorToTransform` _returnvalue)) "AlwaysSpawn" "OverrideRootScale" null ControlledPawn))
        (set `Spell.spellCaster` (cast `MythicismCharacter` ControlledPawn :!pure true) _returnvalue_2)
        (`QuickSpell.FireSpell` _returnvalue_2 (`KismetMathLibrary.Normal` (- (`Actor.K2_GetActorLocation` (`GameplayStatics.GetPlayerCharacter` 0)) _returnvalue)))))
    (else
      (`KismetSystemLibrary.Delay` 0.5)))
  (`self.FinishExecute` true))