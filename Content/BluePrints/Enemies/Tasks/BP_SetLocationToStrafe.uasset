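; Behavior Tree task that picks a point for an Enemy pawn to strafe toward.
; It randomly chooses left or right, then offsets from the enemy's mesh location slightly forward and sideways along the actor's vectors.
; It writes the point to a Blackboard key and sets the enemy's max walk speed to the strafe speed.
; After a short delay it finishes successfully, leaving the movement itself outside this task.
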(event `self.ReceiveExecuteAI`
  (params (OwnerController :type "AIController Object Reference") (ControlledPawn :type "Pawn Object Reference"))
  (bind _asenemy (cast `Enemy` ControlledPawn :!pure true))
  ;[1 1 1] Set Strafe Left or Right
  (if (< (`KismetMathLibrary.RandomInteger` 2) 1)
    (set `self.strafeDistance` -150.0)
    (else
      (set `self.strafeDistance` 150.0)))
  ;[1 1 1] Set Strafe Location
  (set `CharacterMovementComponent.MaxWalkSpeed` (`self.strafeSpeed`) (`Character.CharacterMovement` _asenemy))
  (`BTFunctionLibrary.SetBlackboardValueAsVector` (`self.BBRef_StrafeLocation`) (+ (`SceneComponent.K2_GetComponentLocation` (`Character.Mesh` _asenemy)) (* (`Actor.GetActorForwardVector` ControlledPawn) 50.0) (* (`Actor.GetActorRightVector` ControlledPawn) (`self.strafeDistance`))))
  (`KismetSystemLibrary.Delay` 0.2)
  (`self.FinishExecute` true))