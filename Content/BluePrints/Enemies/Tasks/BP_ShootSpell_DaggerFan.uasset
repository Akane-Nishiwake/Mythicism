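; Behavior tree task in which an enemy has a random chance, weighted toward firing, to cast a three-projectile dagger fan spell.
; After a short delay, a successful roll plays a slowed montage, then a timed delay precedes spawning left, center and right spell actors.
; Each spawn combines the pawn's aim rotation with its current weapon's location.
; A failed roll just waits briefly, and both paths finish as success.
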(event `self.ReceiveExecuteAI`
  (params (OwnerController :type "AIController Object Reference") (ControlledPawn :type "Pawn Object Reference"))
  (bind _asenemy (cast `Enemy` ControlledPawn :!pure true))
  (bind _returnvalue (`KismetMathLibrary.ComposeTransforms` (`KismetMathLibrary.Conv_RotatorToTransform` (`Pawn.GetBaseAimRotation` ControlledPawn)) (`KismetMathLibrary.Conv_VectorToTransform` (`Actor.K2_GetActorLocation` (`MythicismCharacter.GetCurrentWeapon` _asenemy)))))
  ;[1 1 1] Calculate Chance for Spell
  (`KismetSystemLibrary.Delay` 0.75)
  (if (> (`KismetMathLibrary.RandomInteger` 11) 2)
    ;[1 1 1] Shoot Dagger Fan Spell
    (`|PlayMontage` (`Character.Mesh` _asenemy) "/Game/Animations/BorrowedAnimations/Burden_slow_Montage.Burden_slow_Montage" 0.5
      (:`then`
        (`KismetSystemLibrary.Delay` 0.9)
        (`|SpawnActorFromClass` "/Game/BluePrints/SpellsAndCurses/Enemy_DaggerFanSpell_Left.Enemy_DaggerFanSpell_Left_C" _returnvalue "Undefined" "OverrideRootScale" null ControlledPawn)
        (`|SpawnActorFromClass` "/Game/BluePrints/SpellsAndCurses/Enemy_TestSpell_Quick.Enemy_TestSpell_Quick_C" _returnvalue "Undefined" "OverrideRootScale" null ControlledPawn)
        (`|SpawnActorFromClass` "/Game/BluePrints/SpellsAndCurses/Enemy_DaggerFanSpell_Right.Enemy_DaggerFanSpell_Right_C" _returnvalue "Undefined" "OverrideRootScale" null ControlledPawn)))
    (else
      (`KismetSystemLibrary.Delay` 0.5)))
  (`self.FinishExecute` true))