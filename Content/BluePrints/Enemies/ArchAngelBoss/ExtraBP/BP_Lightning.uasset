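; BP_Lightning is a short-lived lightning hazard for the ArchAngel boss that destroys itself one second after spawning.
; Its capsule applies heavy health damage to any MythicismPlayer that begins overlapping it.
; A separate LightningDrop event, not called within this Blueprint, spawns an enlarged lightning blast emitter just below the actor at a random yaw.
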(event `self.ReceiveBeginPlay`
  (`KismetSystemLibrary.Delay` 1.0)
  (`self.K2_DestroyActor`))

(event `LightningDrop`
  (bind (_returnvalue_x _returnvalue_y _returnvalue_z) (`KismetMathLibrary.BreakVector` (`self.K2_GetActorLocation` self)))
  (`GameplayStatics.SpawnEmitterAtLocation` "/Game/InfinityBladeEffects/Effects/FX_Mobile/Lightning/P_LineToPoint_Blast_Lightning_00.P_LineToPoint_Blast_Lightning_00" (`KismetMathLibrary.MakeVector` _returnvalue_x _returnvalue_y (- _returnvalue_z 80.0)) (`KismetMathLibrary.MakeRotator` 0.0 0.0 (`KismetMathLibrary.RandomFloatInRange` 0.0 360.0)) (2.0 2.0 2.0) true "AutoRelease"))

(event `self.Capsule.OnComponentBeginOverlap`
  (params (OverlappedComponent :type "PrimitiveComponent Object Reference") (OtherActor :type "Actor Object Reference") (OtherComp :type "PrimitiveComponent Object Reference") (OtherBodyIndex :type Integer) (bFromSweep :type Boolean) (SweepResult :type "HitResult Structure (by ref)"))
  (bind _asmythicism_player (cast `MythicismPlayer` OtherActor))
  (`MythicismCharacter.TakeDamage` _asmythicism_player 500.0 "HealthDamageType" null))

(fn `UserConstructionScript`)