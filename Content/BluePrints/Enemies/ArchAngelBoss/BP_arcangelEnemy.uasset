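; Archangel boss enemy with a second magic phase that leaves a win portal on death.
; Tick fires a one-time transition at half health: it stops AI logic, grants invincibility and plays a taunt with magic circle, shake and sound.
; After a delay, the controller runs the magic behavior tree and invincibility ends.
; OnDie spawns the portal and scales it with a timeline; SetYaw returns the yaw toward a given actor.
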(event `self.ReceiveTick`
  (params (DeltaSeconds :type "Float (single-precision)"))
  (bind _attributes (`self.attributes`))
  (bind _attributes_2 (`self.attributes`))
  (bind (_returnvalue_x _returnvalue_y _returnvalue_z) (`KismetMathLibrary.BreakVector` (`self.K2_GetActorLocation` self)))
  (bind _returnvalue (`self.K2_GetActorLocation` self))
  (`parent.ReceiveTick` DeltaSeconds)
  (if (<= (`CharacterAttributesComponent.health` _attributes) (/ (`CharacterAttributesComponent.maxHealth` _attributes) 2.0))
    (`/Engine/EditorBlueprintResources/StandardMacros.DoOnce` false
      (:`Completed`
        (bind _asbp_archangel_boss_controller (cast `/Game/BluePrints/Enemies/ArchAngelBoss/BP_ArchangelBoss_Controller` (`AIBlueprintHelperLibrary.GetAIController` self)))
        (set `CharacterAttributesComponent.isInvincible` true _attributes_2)
        (bind _returnvalue_2 (`GameplayStatics.SpawnEmitterAtLocation` "/Game/Particles/FXVarietyPack/P_ky_magicCircle1.P_ky_magicCircle1" (`KismetMathLibrary.MakeVector` _returnvalue_x _returnvalue_y (- _returnvalue_z 80.0))))
        (`GameplayStatics.PlayWorldCameraShake` "/Game/BluePrints/UI/BP_Boss_PhaseChangeShake.BP_Boss_PhaseChangeShake_C" _returnvalue 0.0 3000.0 1.0 true)
        (`GameplayStatics.PlaySoundAtLocation` "/Game/Audio/BossSounds/Boss_HealingPhase_Cue.Boss_HealingPhase_Cue" _returnvalue (struct) 1.0 1.0 0.0 null null null)
        (`BrainComponent.StopLogic` (`AIController.BrainComponent` _asbp_archangel_boss_controller) "change phase")
        (`|PlayMontage` (`self.Mesh`) "/Game/Animations/Retargeted_Serath_Animations/Enemy_EvilLaughTaunt.Enemy_EvilLaughTaunt" 0.7
          (:`then`
            (`KismetSystemLibrary.Delay` 3.0)
            (`AIController.RunBehaviorTree` _asbp_archangel_boss_controller "/Game/BluePrints/Enemies/ArchAngelBoss/ArchangelMagic_Tree.ArchangelMagic_Tree")
            (set `CharacterAttributesComponent.isInvincible` false _attributes_2)
            (`ActorComponent.K2_DestroyComponent` _returnvalue_2)))))))

(event `self.OnDie`
  (bind (_returnvalue_x _returnvalue_y _returnvalue_z) (`KismetMathLibrary.BreakVector` (`self.K2_GetActorLocation` self)))
  (`parent.OnDie`)
  (`KismetSystemLibrary.PrintString` "Boss Defeated" true true (struct :`R` 1.0 :`G` 0.061054 :`B` 0.942253 :`A` 1.0))
  (bind _returnvalue (`|SpawnActorFromClass` "/Game/BluePrints/Interactable/BP_WinPortal.BP_WinPortal_C" (`KismetMathLibrary.MakeTransform` (`KismetMathLibrary.MakeVector` _returnvalue_x _returnvalue_y (- _returnvalue_z 100.0))) "Undefined" "OverrideRootScale" null null))
  (bind (_direction _newtrack_0) (`Timeline|Portal Grow` :!via `PlayFromStart`)
    (:`Update`
      (`self.SetActorScale3D` _returnvalue (`KismetMathLibrary.MakeVector` _newtrack_0 _newtrack_0 _newtrack_0)))))

(fn `SetYaw`
  (params (NewParam :type "Actor Object Reference"))
  (returns (NewParam1 :type "Float (double-precision)"))
  (bind (_returnvalue_roll _returnvalue_pitch _returnvalue_yaw) (`KismetMathLibrary.BreakRotator` (`KismetMathLibrary.FindLookAtRotation` (`self.K2_GetActorLocation`) (`self.K2_GetActorLocation` NewParam))))
  (return _returnvalue_yaw))

(fn `UserConstructionScript`
  (`parent.UserConstructionScript`))