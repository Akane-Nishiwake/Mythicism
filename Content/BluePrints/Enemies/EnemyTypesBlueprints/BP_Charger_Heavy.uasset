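; BP_Charger_Heavy is a heavy Charger enemy Blueprint that adjusts its AI and damage around being airborne.
; When its movement mode changes to Falling, its Charger controller switches to an empty behavior tree to suspend AI logic.
; Any other mode change restarts the Charger behavior tree, and landing from a fall into walking also calls TakeFallDamage.
; Its construction script defers to the parent, and the other events are empty or disabled.
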(event `self.K2_OnMovementModeChanged`
  (params (PrevMovementMode :type "EMovementMode Enum" :default "MOVE_None") (NewMovementMode :type "EMovementMode Enum" :default "MOVE_None") (PrevCustomMode :type Byte) (NewCustomMode :type Byte))
  ;[1 1 1] Airborne Behavior Fix
  (if (`|EnumEquality` NewMovementMode "MOVE_Falling")
    (bind _asbp_enemy_controller_charger (cast `/Game/BluePrints/Enemies/ChargerEnemy/BP_EnemyController_Charger` (`self.GetController`)))
    (`AIController.RunBehaviorTree` _asbp_enemy_controller_charger "/Game/BluePrints/Enemies/MagicEnemy/Tree_Empty.Tree_Empty")
    (else
      (bind _asbp_enemy_controller_charger_2 (cast `/Game/BluePrints/Enemies/ChargerEnemy/BP_EnemyController_Charger` (`self.GetController`)))
      (`AIController.RunBehaviorTree` _asbp_enemy_controller_charger_2 "/Game/BluePrints/Enemies/ChargerEnemy/Enemy_Charger_Tree1.Enemy_Charger_Tree1")
      (if (and (`|EnumEquality` PrevMovementMode "MOVE_Falling") (or (`|EnumEquality` NewMovementMode "MOVE_Walking") (`|EnumEquality` NewMovementMode "MOVE_NavWalking")))
        (`self.TakeFallDamage`)))))

(event `self.ReceiveActorBeginOverlap`
  (params (OtherActor :type "Actor Object Reference"))
  ;[1 1 1] Airborne Behavior Fix
)

(fn `UserConstructionScript`
  (`parent.UserConstructionScript`))