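; BP_Magic_LifeDrain is the character Blueprint for the life-drain magic enemy, adding an airborne behavior fix through movement mode changes.
; When it starts falling, it interrupts its AI controller and swaps in an empty behavior tree.
; Any other movement mode restarts the life-drain behavior tree, and landing from a fall into walking or nav walking also calls TakeFallDamage.
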(event `self.K2_OnMovementModeChanged`
  (params (PrevMovementMode :type "EMovementMode Enum" :default "MOVE_None") (NewMovementMode :type "EMovementMode Enum" :default "MOVE_None") (PrevCustomMode :type Byte) (NewCustomMode :type Byte))
  ;[1 1 1] Airborne Behavior Fix
  (if (`|EnumEquality` NewMovementMode "MOVE_Falling")
    (bind _asbp_magic_enemy_controller_life_drain (cast `/Game/BluePrints/Enemies/MagicEnemy/BP_MagicEnemy_Controller_LifeDrain` (`self.GetController`)))
    (message `/Game/BluePrints/MythicismPlayer/BPI_AnimationTriggerable.Interrupt` _asbp_magic_enemy_controller_life_drain)
    (`AIController.RunBehaviorTree` _asbp_magic_enemy_controller_life_drain "/Game/BluePrints/Enemies/MagicEnemy/Tree_Empty.Tree_Empty")
    (else
      (bind _asbp_magic_enemy_controller_life_drain_2 (cast `/Game/BluePrints/Enemies/MagicEnemy/BP_MagicEnemy_Controller_LifeDrain` (`self.GetController`)))
      (`AIController.RunBehaviorTree` _asbp_magic_enemy_controller_life_drain_2 "/Game/BluePrints/Enemies/MagicEnemy/MagicEnemy_LifeDrain_Tree.MagicEnemy_LifeDrain_Tree")
      (if (and (`|EnumEquality` PrevMovementMode "MOVE_Falling") (or (`|EnumEquality` NewMovementMode "MOVE_NavWalking") (`|EnumEquality` NewMovementMode "MOVE_Walking")))
        (`self.TakeFallDamage`)))))

(fn `UserConstructionScript`
  (`parent.UserConstructionScript`))