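; Player stats Blueprint that holds four levelable attributes: Heart, Body, Mind and Soul.
; Each attribute derives linear multipliers for health, stamina and attack, mana and magic defense, or defense and favor, all set on BeginPlay.
; Level-up events increment an attribute, refresh its multipliers and recalculate its next cost from StartCost and the new level.
; BeginPlay leaves costs uncalculated, and no currency is checked or spent here.
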(event `SetMindMultipliers`
  (bind _mind (`self.Mind`))
  ;[0.822 0.4034 1] Set Multipliers for Mind Stat
  (set `self.ManaMultiplier` (+ 1.0 (* _mind 0.05)))
  (set `self.MagicDefMultiplier` (* _mind 5.0)))

(event `SetSoulMultipliers`
  (bind _soul (`self.Soul`))
  ;[0.822 0.4034 1] Set Multipliers for Soul Stat
  (set `self.DefMultiplier` (* _soul 3.0))
  (set `self.FavorMultiplier` (+ (* _soul 0.1) 1.0)))

(event `SetHeartMultipliers`
  ;[0.822 0.4034 1] Set Multipliers for Heart Stat
  (set `self.HealthMultiplier` (+ 1.0 (* (`self.Heart`) 0.05))))

(event `SetBodyMultipliers`
  (bind _body (`self.Body`))
  ;[0.822 0.4034 1] Set Multipliers for Body Stat
  (set `self.StaminaMultiplier` (+ 1.0 (* _body 0.05)))
  (set `self.AtkMultiplier` (* _body 5.0)))

(event `self.ReceiveBeginPlay`
  ;[0.1599 0.7261 1] Initialize multipliers based on level
  (`self.SetHeartMultipliers`)
  (`self.SetBodyMultipliers`)
  (`self.SetMindMultipliers`)
  (`self.SetSoulMultipliers`))

(event `HeartLevelCost`
  ;[1 0.619 0.1563] Set cost for next Heart level
  (set `self.HeartNextCost` (`KismetMathLibrary.FTrunc` (* (`self.startCost`) (* (`self.Heart`) 1.1)))))

(event `LevelUpHeart`
  ;[0.3032 1 0.1758] Level Up Heart
  (`/Engine/EditorBlueprintResources/StandardMacros.IncrementInt` (`self.Heart`)
    (:`  `
      (`self.SetHeartMultipliers`)
      (`self.HeartLevelCost`))))

(event `LevelUpMind`
  ;[0.3032 1 0.1758] Level Up Mind
  (`/Engine/EditorBlueprintResources/StandardMacros.IncrementInt` (`self.Mind`)
    (:`  `
      (`self.SetMindMultipliers`)
      (`self.MindLevelCost`))))

(event `BodyLevelCost`
  ;[1 0.619 0.1563] Set cost for next Body level
  (set `self.BodyNextCost` (`KismetMathLibrary.FTrunc` (* (`self.startCost`) (* (`self.Body`) 1.1)))))

(event `LevelUpBody`
  ;[0.3032 1 0.1758] Level Up Body
  (`/Engine/EditorBlueprintResources/StandardMacros.IncrementInt` (`self.Body`)
    (:`  `
      (`self.SetBodyMultipliers`)
      (`self.BodyLevelCost`))))

(event `LevelUpSoul`
  ;[0.3032 1 0.1758] Level Up Soul
  (`/Engine/EditorBlueprintResources/StandardMacros.IncrementInt` (`self.Soul`)
    (:`  `
      (`self.SetSoulMultipliers`)
      (`self.SoulLevelCost`))))

(event `MindLevelCost`
  ;[1 0.619 0.1563] Set cost for next Mind level
  (set `self.MindNextCost` (`KismetMathLibrary.FTrunc` (* (`self.startCost`) (* (`self.Mind`) 1.1)))))

(event `SoulLevelCost`
  ;[1 0.619 0.1563] Set cost for next Soul level
  (set `self.SoulNextCost` (`KismetMathLibrary.FTrunc` (* (`self.startCost`) (* (`self.Soul`) 1.1)))))