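; Actor component that spawns blood splatter effects at its owning actor, through a single SpawnBloodsplatter function.
; It plays a cone splat particle with a random roll to either side, scaled by SplatScale with a floor of one.
; A long downward visibility trace, ignoring the owner, places a BP_BloodDecal actor with random yaw and DecalScale, without checking for a hit.
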(fn `SpawnBloodsplatter`
  (params (SplatScale :type "Float (double-precision)" :default 1.0) (DecalScale :type "Float (double-precision)" :default 1.0))
  (bind _returnvalue (`self.GetOwner`))
  (bind (_returnvalue_x _returnvalue_y _returnvalue_z) (`KismetMathLibrary.BreakVector` (`Actor.K2_GetActorLocation` _returnvalue)))
  ;[1 1 1] Splat particle
  (`GameplayStatics.SpawnEmitterAtLocation` "/Game/Particles/Realistic_Starter_VFK_Pack_Vol2/Particles/Blood/P_Blood_Splat_Cone.P_Blood_Splat_Cone" (`Actor.K2_GetActorLocation` (`self.GetOwner`)) (`KismetMathLibrary.MakeRotator` (* (- (* (`KismetMathLibrary.RandomInteger` 2) 2) 1) (`KismetMathLibrary.RandomFloatInRange` 10.0 50.0))) (`KismetMathLibrary.Conv_DoubleToVector` (`KismetMathLibrary.FMax` SplatScale 1.0)))
  ;[1 1 1] Decal
  (bind _outhit (`KismetSystemLibrary.LineTraceSingle` (`KismetMathLibrary.MakeVector` _returnvalue_x _returnvalue_y _returnvalue_z) (`KismetMathLibrary.MakeVector` _returnvalue_x _returnvalue_y (- _returnvalue_z 5000.0)) "TraceTypeQuery1" false (`|MakeArray` _returnvalue)))
  (`|SpawnActorFromClass` "/Game/Materials/WeaponTrails/BP_BloodDecal.BP_BloodDecal_C" (`KismetMathLibrary.MakeTransform` (`.Location` (`GameplayStatics.BreakHitResult` _outhit)) (`KismetMathLibrary.MakeRotator` 0.0 0.0 (`KismetMathLibrary.RandomFloatInRange` 0.0 360.0)) (`KismetMathLibrary.Conv_DoubleToVector` DecalScale)) "Undefined" "OverrideRootScale" null null))