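; BP_Spikes is a hazard that makes falls more punishing for enemies and the player while they overlap it.
; Begin overlap lowers fall damage velocity thresholds and sets higher multipliers, also lowers the enemy ragdoll threshold, and prints a debug message.
; End overlap writes hard-coded values back instead of cached originals, except the enemy multiplier, which is derived from movement mass.
; The spikes apply no damage directly.
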(event `self.ReceiveActorEndOverlap`
  (params (OtherActor :type "Actor Object Reference"))
  ;[1 1 1] Leava the spike
  (bind _asbp_enemy_1_character (cast `/Game/BluePrints/Enemies/BP_Enemy_1_Character` OtherActor)
    (:`then`
      (set `/Game/BluePrints/Enemies/BP_Enemy_1_Character.FallDamageMultiplier` (/ (`CharacterMovementComponent.Mass` (`Character.CharacterMovement` _asbp_enemy_1_character)) 100.0) _asbp_enemy_1_character)
      (set `/Game/BluePrints/Enemies/BP_Enemy_1_Character.FallDamageVelocityThreshold` 1500.0 _asbp_enemy_1_character)
      (set `/Game/BluePrints/Enemies/BP_Enemy_1_Character.RagdollVelocityThreshold` 650.0 _asbp_enemy_1_character))
    (:`CastFailed`
      (bind _asbp_mythicism_player (cast `/Game/BluePrints/MythicismPlayer/BP_MythicismPlayer` OtherActor))
      (set `/Game/BluePrints/MythicismPlayer/BP_MythicismPlayer.FallDamageVelocityThreshold` 1750.0 _asbp_mythicism_player)
      (set `/Game/BluePrints/MythicismPlayer/BP_MythicismPlayer.FallDamageMultiplier` 1.0 _asbp_mythicism_player))))

(event `self.ReceiveActorBeginOverlap`
  (params (OtherActor :type "Actor Object Reference"))
  ;[1 1 1] Toucha the spike
  (bind _asbp_enemy_1_character (cast `/Game/BluePrints/Enemies/BP_Enemy_1_Character` OtherActor)
    (:`then`
      (set `/Game/BluePrints/Enemies/BP_Enemy_1_Character.FallDamageMultiplier` 2.0 _asbp_enemy_1_character)
      (set `/Game/BluePrints/Enemies/BP_Enemy_1_Character.FallDamageVelocityThreshold` 500.0 _asbp_enemy_1_character)
      (set `/Game/BluePrints/Enemies/BP_Enemy_1_Character.RagdollVelocityThreshold` 300.0 _asbp_enemy_1_character)
      (`KismetSystemLibrary.PrintString` "get spiked lmao"))
    (:`CastFailed`
      (bind _asbp_mythicism_player (cast `/Game/BluePrints/MythicismPlayer/BP_MythicismPlayer` OtherActor))
      (set `/Game/BluePrints/MythicismPlayer/BP_MythicismPlayer.FallDamageVelocityThreshold` 500.0 _asbp_mythicism_player)
      (set `/Game/BluePrints/MythicismPlayer/BP_MythicismPlayer.FallDamageMultiplier` 1.5 _asbp_mythicism_player)
      (`KismetSystemLibrary.PrintString` "oof"))))

(fn `UserConstructionScript`)