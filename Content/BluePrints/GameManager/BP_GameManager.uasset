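; Game manager that turns player input into quick-swap scrolling, inventory menu control, gamepad detection and consumable use.
; It reaches the quick-swap, inventory and HUD widgets through ThirdPersonGameMode, disabling pawn input while the inventory is open.
; Consumables route by type through feedback graphs into UseConsumable, which decrements counts, applies effects and refreshes UI.
; It also silently adds items, though consumables reach only the UI, and prints a win message when enemies run out.
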(event `InputAction|ConsumableSwap`
  (params (Key :type "Key Structure"))
  ;[0.256 1 0.435] Iterate Equipment Slots
  (:`Pressed`
    (`GameplayStatics.PlaySound2D` "/Game/Audio/UI/UI_Click.UI_Click" 1.0 1.0 0.0 null null)
    (bind _asthird_person_game_mode (cast `/Game/BluePrints/ThirdPersonCharacter/ThirdPersonGameMode` (`GameplayStatics.GetGameMode`)))
    (`/Game/BluePrints/UI/Inventory/BP_QuickSwap_UI.ScrollConsumable` (`/Game/BluePrints/ThirdPersonCharacter/ThirdPersonGameMode.QuickSwapWidget` _asthird_person_game_mode))))

(event `InputAction|SpellSwap`
  (params (Key :type "Key Structure"))
  ;[0.256 1 0.435] Iterate Equipment Slots
  (:`Pressed`
    (`GameplayStatics.PlaySound2D` "/Game/Audio/UI/UI_Click.UI_Click" 1.0 1.0 0.0 null null)
    (bind _asthird_person_game_mode (cast `/Game/BluePrints/ThirdPersonCharacter/ThirdPersonGameMode` (`GameplayStatics.GetGameMode`)))
    (`/Game/BluePrints/UI/Inventory/BP_QuickSwap_UI.ScrollSpell` (`/Game/BluePrints/ThirdPersonCharacter/ThirdPersonGameMode.QuickSwapWidget` _asthird_person_game_mode))))

(event `InputAction|AnyKey` :consume false
  (params (Key :type "Key Structure"))
  (bind _returnvalue (`KismetInputLibrary.Key_IsGamepadKey` Key))
  (bind _returnvalue_2 (`GameplayStatics.GetGameMode`))
  ;[1 0.1592 0.07955] Detect Controller
  (:`Pressed`
    (if _returnvalue
      (bind _asthird_person_game_mode (cast `/Game/BluePrints/ThirdPersonCharacter/ThirdPersonGameMode` _returnvalue_2))
      (set `/Game/BluePrints/ThirdPersonCharacter/ThirdPersonGameMode.IsUsingController` _returnvalue _asthird_person_game_mode)
      (else
        (bind _asthird_person_game_mode_2 (cast `/Game/BluePrints/ThirdPersonCharacter/ThirdPersonGameMode` _returnvalue_2))
        (set `/Game/BluePrints/ThirdPersonCharacter/ThirdPersonGameMode.IsUsingController` _returnvalue _asthird_person_game_mode_2)))))

(event `CallToggleInventory`
  (bind _returnvalue (`GameplayStatics.GetPlayerController` 0))
  (bind _returnvalue_2 (`GameplayStatics.GetPlayerPawn` 0))
  ;[0.2784 0.1686 1] Show / Hide Inventory UI
  (bind _output_get (set `self.IsInventoryOpen` (not (`self.IsInventoryOpen`))))
  (bind _asthird_person_game_mode (cast `/Game/BluePrints/ThirdPersonCharacter/ThirdPersonGameMode` (`GameplayStatics.GetGameMode`)))
  (`/Game/BluePrints/ThirdPersonCharacter/ThirdPersonGameMode.InventoryToggle` _asthird_person_game_mode)
  (if _output_get
    (bind _asmythicism_player (cast `MythicismPlayer` _returnvalue_2))
    (`self.DisableInput` _returnvalue_2 _returnvalue)
    (`self.DisableInput` _asmythicism_player _returnvalue)
    (else
      (bind _asmythicism_player_2 (cast `MythicismPlayer` _returnvalue_2))
      (`self.EnableInput` _returnvalue_2 _returnvalue)
      (`self.EnableInput` _asmythicism_player_2 _returnvalue))))

(event `InputAction|WeaponSwap`
  (params (Key :type "Key Structure"))
  ;[0.256 1 0.435] Iterate Equipment Slots
  (:`Pressed`
    (`GameplayStatics.PlaySound2D` "/Game/Audio/UI/UI_Click.UI_Click" 1.0 1.0 0.0 null null)
    (bind _asthird_person_game_mode (cast `/Game/BluePrints/ThirdPersonCharacter/ThirdPersonGameMode` (`GameplayStatics.GetGameMode`)))
    (`/Game/BluePrints/UI/Inventory/BP_QuickSwap_UI.ScrollWeapon` (`/Game/BluePrints/ThirdPersonCharacter/ThirdPersonGameMode.QuickSwapWidget` _asthird_person_game_mode))))

(event `InputAction|Jump` :consume false
  (params (Key :type "Key Structure"))
  ;[0.2784 0.1686 1] Inventory Menu Controls
  (:`Pressed`
    (if (`self.IsInventoryOpen`)
      (if (`KismetInputLibrary.Key_IsGamepadKey` Key)
        _))))

(event `Key|Gamepad_LeftShoulder` :consume false
  (params (Key :type "Key Structure"))
  ;[0.2784 0.1686 1] Inventory Menu Controls
  (:`Pressed`
    (if (`self.IsInventoryOpen`)
      (bind _asthird_person_game_mode (cast `/Game/BluePrints/ThirdPersonCharacter/ThirdPersonGameMode` (`GameplayStatics.GetGameMode`)))
      (`/Game/BluePrints/UI/Inventory/BP_InventoryUI.PreviousPanel` (`/Game/BluePrints/ThirdPersonCharacter/ThirdPersonGameMode.InventoryWidget` _asthird_person_game_mode)))))

(event `Key|Gamepad_RightShoulder` :consume false
  (params (Key :type "Key Structure"))
  ;[0.2784 0.1686 1] Inventory Menu Controls
  (:`Pressed`
    (if (`self.IsInventoryOpen`)
      (bind _asthird_person_game_mode (cast `/Game/BluePrints/ThirdPersonCharacter/ThirdPersonGameMode` (`GameplayStatics.GetGameMode`)))
      (`/Game/BluePrints/UI/Inventory/BP_InventoryUI.NextPanel` (`/Game/BluePrints/ThirdPersonCharacter/ThirdPersonGameMode.InventoryWidget` _asthird_person_game_mode)))))

(event `InputAction|Inventory`
  (params (Key :type "Key Structure"))
  ;[0.2784 0.1686 1] Inventory Menu Controls
  (:`Pressed`
    (`WidgetBlueprintLibrary.SetFocusToGameViewport`)
    (`self.CallToggleInventory`)))

(event `InputAction|Menu` :consume false
  (params (Key :type "Key Structure"))
  ;[0.2784 0.1686 1] Inventory Menu Controls
  (:`Pressed`
    (if (`self.IsInventoryOpen`)
      (`self.CallToggleInventory`))))

(event `SilentlyAddItemToInventory`
  (params (Item :type "Item Object Reference"))
  ;[0.2784 0.1686 1] Silent Add Item
  (bind _returnvalue (`GameplayStatics.GetActorOfClass` "/Game/BluePrints/MythicismPlayer/BP_MythicismPlayer.BP_MythicismPlayer_C"))
  (bind _asweapon_item (cast `WeaponItem` Item)
    (:`then`
      (bind _returnvalue_2 (`self.GetComponentByClass` _returnvalue "/Script/Mythicism.Inventory"))
      (`Inventory.AddWeapon` _returnvalue_2 _asweapon_item)
      (bind _asthird_person_game_mode (cast `/Game/BluePrints/ThirdPersonCharacter/ThirdPersonGameMode` (`GameplayStatics.GetGameMode`)))
      (`/Game/BluePrints/UI/Inventory/BP_InventoryUI.AddWeaponToUI` (`/Game/BluePrints/ThirdPersonCharacter/ThirdPersonGameMode.InventoryWidget` _asthird_person_game_mode) _asweapon_item))
    (:`CastFailed`
      (bind _asspell_item (cast `SpellItem` Item)
        (:`then`
          (`Inventory.AddSpell` _returnvalue_2 _asspell_item)
          (bind _asthird_person_game_mode_2 (cast `/Game/BluePrints/ThirdPersonCharacter/ThirdPersonGameMode` (`GameplayStatics.GetGameMode`)))
          (`/Game/BluePrints/UI/Inventory/BP_InventoryUI.AddSpellToUI` (`/Game/BluePrints/ThirdPersonCharacter/ThirdPersonGameMode.InventoryWidget` _asthird_person_game_mode_2) _asspell_item))
        (:`CastFailed`
          (bind _askey_item (cast `KeyItem` Item)
            (:`then`
              (`Inventory.AddKey` _returnvalue_2 _askey_item)
              (bind _asthird_person_game_mode_3 (cast `/Game/BluePrints/ThirdPersonCharacter/ThirdPersonGameMode` (`GameplayStatics.GetGameMode`)))
              (`/Game/BluePrints/UI/Inventory/BP_InventoryUI.AddKeyToUI` (`/Game/BluePrints/ThirdPersonCharacter/ThirdPersonGameMode.InventoryWidget` _asthird_person_game_mode_3) _askey_item))
            (:`CastFailed`
              (bind _asconsumable_item (cast `ConsumableItem` Item))
              (bind _asthird_person_game_mode_4 (cast `/Game/BluePrints/ThirdPersonCharacter/ThirdPersonGameMode` (`GameplayStatics.GetGameMode`)))
              (`/Game/BluePrints/UI/Inventory/BP_InventoryUI.AddConsumableToUI` (`/Game/BluePrints/ThirdPersonCharacter/ThirdPersonGameMode.InventoryWidget` _asthird_person_game_mode_4) _asconsumable_item))))))))

(event `InputAction|Roll` :consume false
  (params (Key :type "Key Structure"))
  ;[0.2784 0.1686 1] Inventory Menu Controls
  (:`Pressed`
    (if (`self.IsInventoryOpen`)
      (`self.CallToggleInventory`))))

(event `InputAction|Consumable`
  (params (Key :type "Key Structure"))
  (bind _attributes (`MythicismCharacter.attributes` (`self.player`)))
  ;[1 0.1583 0.9096] Consumables
  (:`Pressed`
    (bind _asthird_person_game_mode (cast `/Game/BluePrints/ThirdPersonCharacter/ThirdPersonGameMode` (`GameplayStatics.GetGameMode`)))
    (bind _asbp_mythicism_player (cast `/Game/BluePrints/MythicismPlayer/BP_MythicismPlayer` (`GameplayStatics.GetPlayerCharacter` 0)))
    (set `self.player` _asbp_mythicism_player)
    (bind _quickswapwidget (`/Game/BluePrints/ThirdPersonCharacter/ThirdPersonGameMode.QuickSwapWidget` _asthird_person_game_mode))
    (bind _output (`|GetArrayItem` (`/Game/BluePrints/UI/Inventory/BP_QuickSwap_UI.ConsumableData` _quickswapwidget) (`/Game/BluePrints/UI/Inventory/BP_QuickSwap_UI.ConsumableIndex` _quickswapwidget)))
    (if (`KismetSystemLibrary.IsValid` _output)
      (switch `EConsumableType` (`Consumable.ConsumableType` (`ConsumableItem.ConsumableData` _output))
        (:`HealthPotion`
          (if (== (`CharacterAttributesComponent.health` _attributes) (`CharacterAttributesComponent.maxHealth` _attributes))
            (`GameplayStatics.PlaySound2D` "/Game/Audio/UI/UI_Error_Cue.UI_Error_Cue" 1.0 1.0 0.0 null null :!label _label)
            (else
              (`self.UseConsumable` _output)
              (bind _asthird_person_game_mode_2 (cast `/Game/BluePrints/ThirdPersonCharacter/ThirdPersonGameMode` (`GameplayStatics.GetGameMode`)))
              (`/Game/BluePrints/UI/PlayerHud/BP_PlayerHud.FillHealth` (`/Game/BluePrints/ThirdPersonCharacter/ThirdPersonGameMode.HUDWidget` _asthird_person_game_mode_2))
              (`GameplayStatics.PlaySound2D` "/Game/Audio/UI/Inventory/HealHealth_Cue.HealHealth_Cue" 1.0 1.0 0.0 null null)
              (`GameplayStatics.PlaySound2D` "/Game/Audio/UI/Inventory/Human_Drinking_Cue.Human_Drinking_Cue" 1.0 1.0 0.0 null null)
              (bind _returnvalue (`GameplayStatics.SpawnEmitterAttached` "/Game/Particles/FXVarietyPack/P_FillHealthAura1.P_FillHealthAura1" (`Character.CapsuleComponent` (`self.player`)) "None" (0.0 0.0 0.0) (struct) (0.3 0.3 0.3)))
              (`KismetSystemLibrary.Delay` 0.7)
              (`ActorComponent.K2_DestroyComponent` _returnvalue))))
        (:`ManaPotion`
          (if (== (`CharacterAttributesComponent.mana` _attributes) (`CharacterAttributesComponent.maxMana` _attributes))
            (goto _label)
            (else
              (`self.UseConsumable` _output)
              (bind _asthird_person_game_mode_3 (cast `/Game/BluePrints/ThirdPersonCharacter/ThirdPersonGameMode` (`GameplayStatics.GetGameMode`)))
              (`/Game/BluePrints/UI/PlayerHud/BP_PlayerHud.FillMana` (`/Game/BluePrints/ThirdPersonCharacter/ThirdPersonGameMode.HUDWidget` _asthird_person_game_mode_3))
              (`GameplayStatics.PlaySound2D` "/Game/Audio/UI/Inventory/HealMana_Cue.HealMana_Cue" 1.0 1.0 0.0 null null)
              (`GameplayStatics.PlaySound2D` "/Game/Audio/UI/Inventory/Human_Drinking_Cue.Human_Drinking_Cue" 1.0 1.0 0.0 null null)
              (bind _returnvalue_2 (`GameplayStatics.SpawnEmitterAttached` "/Game/Particles/FXVarietyPack/P_FillManaAura.P_FillManaAura" (`Character.CapsuleComponent` (`self.player`)) "None" (0.0 0.0 0.0) (struct) (0.3 0.3 0.3)))
              (`KismetSystemLibrary.Delay` 1.0)
              (`ActorComponent.K2_DestroyComponent` _returnvalue_2))))
        (:`InstantFavor`
          (`self.UseConsumable` _output))
        (:`SpeedBoost`
          (`self.UseConsumable` _output)
          (`GameplayStatics.PlaySound2D` "/Game/Audio/UI/UI_Click.UI_Click" 1.0 1.0 0.0 null null)
          (`GameplayStatics.PlaySound2D` "/Game/Audio/UI/Inventory/UseRabbitPotion_Cue.UseRabbitPotion_Cue" 1.0 1.0 0.0 null null)
          (bind _returnvalue_3 (`GameplayStatics.SpawnEmitterAttached` "/Game/Particles/FXVarietyPack/P_SpeedAura.P_SpeedAura" (`Character.CapsuleComponent` (`self.player`)) "None" (0.0 0.0 0.0) (struct) (0.3 0.3 0.3)))
          (`KismetSystemLibrary.Delay` 1.0)
          (`ActorComponent.K2_DestroyComponent` _returnvalue_3)))
      (else
        (goto _label)))))

(event `UseConsumable`
  (params (Consumable :type "ConsumableItem Object Reference (by ref)"))
  (bind _consumabledata (`ConsumableItem.ConsumableData` Consumable))
  (bind _player (`self.player`))
  (bind _returnvalue (`KismetMathLibrary.Conv_IntToDouble` (`Consumable.amount` _consumabledata)))
  ;[1 0.1583 0.9096] Consumables
  (bind _asbp_mythicism_player (cast `/Game/BluePrints/MythicismPlayer/BP_MythicismPlayer` (`GameplayStatics.GetPlayerCharacter` 0)))
  (set `self.player` _asbp_mythicism_player)
  (bind _used (`self.Check Consumable Count` Consumable))
  (if _used
    (switch `EConsumableType` (`Consumable.ConsumableType` _consumabledata)
      (:`HealthPotion`
        (bind _asbp_mythicism_player_2 (cast `/Game/BluePrints/MythicismPlayer/BP_MythicismPlayer` (`GameplayStatics.GetPlayerPawn` 0)))
        (`MythicismCharacter.Heal` _asbp_mythicism_player_2 _returnvalue "HealthDamageType")
        (bind _asthird_person_game_mode (cast `/Game/BluePrints/ThirdPersonCharacter/ThirdPersonGameMode` (`GameplayStatics.GetGameMode`) :!label _label_2))
        (bind _quickswapwidget (`/Game/BluePrints/ThirdPersonCharacter/ThirdPersonGameMode.QuickSwapWidget` _asthird_person_game_mode))
        (`/Game/BluePrints/UI/Inventory/BP_QuickSwap_UI.RedrawConsumableCount` _quickswapwidget (`ConsumableItem.Count` (`|GetArrayItem` (`/Game/BluePrints/UI/Inventory/BP_QuickSwap_UI.ConsumableData` _quickswapwidget) (`/Game/BluePrints/UI/Inventory/BP_QuickSwap_UI.ConsumableIndex` _quickswapwidget))))
        ;;[1 1 1] Update count in inventory
        (bind _consumablewidget (`/Game/BluePrints/UI/Inventory/BP_InventoryUI.Find Consumable Widget` (`/Game/BluePrints/ThirdPersonCharacter/ThirdPersonGameMode.InventoryWidget` _asthird_person_game_mode) Consumable))
        (`TextBlock.SetText` (`/Game/BluePrints/UI/Inventory/BP_InventoryConsumableUI.CountText` _consumablewidget) (`KismetTextLibrary.Conv_StringToText` (`KismetStringLibrary.Concat_StrStr` "x" (`KismetTextLibrary.Conv_TextToString` (`KismetTextLibrary.Conv_IntToText` (`ConsumableItem.Count` Consumable)))))))
      (:`ManaPotion`
        (bind _asbp_mythicism_player_3 (cast `/Game/BluePrints/MythicismPlayer/BP_MythicismPlayer` (`GameplayStatics.GetPlayerPawn` 0)))
        (`MythicismCharacter.Heal` _asbp_mythicism_player_3 _returnvalue "ManaDamageType")
        (goto _label_2))
      (:`InstantFavor`
        ;;[1 1 1] Use favor consumable
        (bind _asthird_person_game_mode_2 (cast `/Game/BluePrints/ThirdPersonCharacter/ThirdPersonGameMode` (`GameplayStatics.GetGameMode`)))
        (`/Game/BluePrints/ThirdPersonCharacter/ThirdPersonGameMode.AddFavor` _asthird_person_game_mode_2 (`KismetMathLibrary.Conv_IntToDouble` (`Consumable.amount` (`ConsumableItem.ConsumableData` Consumable))))
        (if (> (`ConsumableItem.Count` Consumable) 0)
          (goto _label_2)
          (else
            ;;[1 0.8436 0] Delete An Empty Consumable
            (bind _asthird_person_game_mode_3 (cast `/Game/BluePrints/ThirdPersonCharacter/ThirdPersonGameMode` (`GameplayStatics.GetGameMode`)))
            (bind _consumablewidget_2 (`/Game/BluePrints/UI/Inventory/BP_InventoryUI.Find Consumable Widget` (`/Game/BluePrints/ThirdPersonCharacter/ThirdPersonGameMode.InventoryWidget` _asthird_person_game_mode_3) Consumable))
            (bind _quickswapwidget_2 (`/Game/BluePrints/ThirdPersonCharacter/ThirdPersonGameMode.QuickSwapWidget` _asthird_person_game_mode_3))
            (`/Game/BluePrints/UI/Inventory/BP_QuickSwap_UI.RedrawConsumableCount` _quickswapwidget_2 (`ConsumableItem.Count` (`|GetArrayItem` (`/Game/BluePrints/UI/Inventory/BP_QuickSwap_UI.ConsumableData` _quickswapwidget_2) (`/Game/BluePrints/UI/Inventory/BP_QuickSwap_UI.ConsumableIndex` _quickswapwidget_2))))
            (`/Game/BluePrints/UI/Inventory/BP_InventoryConsumableUI.DeleteThis` _consumablewidget_2))))
      (:`SpeedBoost`
        (set `/Game/BluePrints/MythicismPlayer/BP_MythicismPlayer.FallDamageVelocityThreshold` 999999.0 _player)
        (set `CharacterMovementComponent.MaxWalkSpeed` 1500.0 (`Character.CharacterMovement` _player))
        (goto _label_2)))
    (else
      (goto _label_2))))

(fn `Check Consumable Count`
  (params (Consumable :type "ConsumableItem Object Reference"))
  (returns (Used :type Boolean))
  (bind _count (`ConsumableItem.Count` Consumable))
  (if (> _count 0)
    (set `ConsumableItem.Count` (- _count 1) Consumable)
    (return true)
    (else
      (`GameplayStatics.PlaySound2D` "/Game/Audio/UI/UI_Error_Cue.UI_Error_Cue" 1.0 1.0 0.0 null null)
      (return false))))

(fn `OnRep_NumberOfEnemies`
  (if (<= (`self.NumberOfEnemies`) 0)
    (`KismetSystemLibrary.PrintString` "YOU WIN")))

(fn `SetCount`
  (params (newCount :type Integer) (Consumable :type "ConsumableItem Object Reference")))

(fn `UserConstructionScript`)