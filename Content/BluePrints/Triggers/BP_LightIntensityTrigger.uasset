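; Trigger actor that fades the level's SkyLight intensity toward a goal value when the MythicismPlayer overlaps it.
; BeginPlay finds the SkyLight and scales the FadeLight timeline's play rate by the inverse of LerpTime.
; On overlap it toggles shadow casting by whether the goal exceeds a fixed threshold.
; The timeline then sets intensity by offsetting the goal with the captured difference scaled by its track.
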(event `self.ReceiveBeginPlay`
  (bind _returnvalue (`GameplayStatics.GetActorOfClass` "/Script/Engine.SkyLight"))
  (set `self.Light` _returnvalue)
  (`TimelineComponent.SetPlayRate` (`self.FadeLight`) (/ 1.0 (`self.LerpTime`))))

(event `self.ReceiveActorBeginOverlap`
  (params (OtherActor :type "Actor Object Reference"))
  (bind _lightcomponent (`SkyLight.LightComponent` (`self.Light`)))
  (cast `MythicismPlayer` OtherActor)
  (set `self.Diff` (- (`self.GoalIntensity`) (`LightComponentBase.Intensity` (`SkyLight.LightComponent` (`self.Light`)))))
  (if (> (`self.GoalIntensity`) 15.0)
    (`LightComponentBase.SetCastShadows` _lightcomponent true)
    (bind (_direction _newtrack_0) (`Timeline|FadeLight` :!label _label)
      (:`Update`
        (`SkyLightComponent.SetIntensity` _lightcomponent (- (`self.GoalIntensity`) (* _newtrack_0 (`self.Diff`))))))
    (else
      (`LightComponentBase.SetCastShadows` _lightcomponent false)
      (goto _label))))

(fn `UserConstructionScript`)