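; Elevator actor that moves its static mesh vertically between two endpoints when BP_MythicismPlayer stands on its button.
; Capsule overlap plays a button-movement timeline, which starts the lift on completion if idle; leaving early stops it.
; A motion timeline, rate-scaled by Time, offsets the mesh from its starting position by up to Distance.
; The GoingUp flag picks forward or reverse playback and is meant to alternate each trip.
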(event `Start`
  (set `self.Idle` false)
  (if (`self.GoingUp`)
    (bind (_direction _movement) (`Timeline|Timeline_Motion` :!label _label)
      (:`Update`
        (bind _output_get (set `self.Height` _movement))
        (`SceneComponent.K2_SetWorldLocation` (`self.StaticMeshComponent`) (+ (`KismetMathLibrary.MakeVector` 0.0 0.0 (* _output_get (`self.Distance`))) (`self.StartPosition`)) false false))
      (:`Finished`
        (set `self.Idle` true)
        (set `self.GoingUp` (not (`self.GoingUp`)))))
    (else
      (goto _label :!via `ReverseFromEnd`))))

(event `LowerButton`
  (set `self.ButtonPressed` true)
  (bind (_direction _newtrack_0) (`Timeline|Timeline_Button` :!via `PlayFromStart` :!label _label_2)
    (:`Update`
      (bind _output_get (set `self.ButtonHeight` _newtrack_0))
      (`SceneComponent.K2_SetRelativeLocation` (`self.Button`) (`KismetMathLibrary.MakeVector` 0.0 0.0 (+ (* _output_get 80.0) 100.0)) false true))
    (:`Finished`
      (if (and (`self.Idle`) (`self.ButtonPressed`))
        (`self.Start`)))))

(event `RaiseButton`
  (set `self.ButtonPressed` false)
  (goto _label_2 :!via `Stop`))

(event `self.ReceiveBeginPlay`
  (`TimelineComponent.SetPlayRate` (`self.Timeline_Button`) 1.0)
  (`TimelineComponent.SetPlayRate` (`self.Timeline_Motion`) (/ 1.0 (`self.Time`)))
  (set `self.StartPosition` (`SceneComponent.K2_GetComponentLocation` (`self.StaticMeshComponent`)))
  (if (`self.GoingUp`)
    (set `self.Height` 0.0)
    (else
      (set `self.Height` 1.0))))

(event `self.Capsule.OnComponentBeginOverlap`
  (params (OverlappedComponent :type "PrimitiveComponent Object Reference") (OtherActor :type "Actor Object Reference") (OtherComp :type "PrimitiveComponent Object Reference") (OtherBodyIndex :type Integer) (bFromSweep :type Boolean) (SweepResult :type "HitResult Structure (by ref)"))
  (cast `/Game/BluePrints/MythicismPlayer/BP_MythicismPlayer` OtherActor)
  (`self.LowerButton`))

(event `self.Capsule.OnComponentEndOverlap`
  (params (OverlappedComponent :type "PrimitiveComponent Object Reference") (OtherActor :type "Actor Object Reference") (OtherComp :type "PrimitiveComponent Object Reference") (OtherBodyIndex :type Integer))
  (cast `/Game/BluePrints/MythicismPlayer/BP_MythicismPlayer` OtherActor)
  (`self.RaiseButton`))

(fn `UserConstructionScript`)