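; One-shot tutorial trigger actor that shows a tutorial popup and pauses the game when the Mythicism player overlaps it.
; It creates a BP_Tutorial widget, fills it with gamepad or keyboard text based on the game mode's controller flag, and switches to Game and UI input.
; Left mouse or gamepad bottom face button unpauses, restores game-only input, removes the widget, forces garbage collection and destroys the trigger.
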(event `self.ReceiveActorBeginOverlap`
  (params (OtherActor :type "Actor Object Reference"))
  (bind _returnvalue (`GameplayStatics.GetPlayerController` 0))
  (bind _tutorialwidget (`self.TutorialWidget`))
  ;[1 1 1] overlap
  (cast `/Game/BluePrints/MythicismPlayer/BP_MythicismPlayer` OtherActor)
  (bind _returnvalue_2 (`|CreateWidget` "/Game/BluePrints/UI/PlayerHud/BP_Tutorial.BP_Tutorial_C" (`GameplayStatics.GetPlayerController` 0)))
  (set `self.TutorialWidget` _returnvalue_2)
  (`UserWidget.AddToViewport` _returnvalue_2 0)
  (bind _asthird_person_game_mode (cast `/Game/BluePrints/ThirdPersonCharacter/ThirdPersonGameMode` (`GameplayStatics.GetGameMode`)))
  (if (`/Game/BluePrints/ThirdPersonCharacter/ThirdPersonGameMode.IsUsingController` _asthird_person_game_mode)
    (`/Game/BluePrints/UI/PlayerHud/BP_Tutorial.PopUpText` _tutorialwidget (`self.gamepadEText`) (`self.gamepadLText`))
    (`WidgetBlueprintLibrary.SetInputMode_GameAndUIEx` _returnvalue null)
    (`GameplayStatics.SetGamePaused` true)
    (else
      (`/Game/BluePrints/UI/PlayerHud/BP_Tutorial.PopUpText` _tutorialwidget (`self.kbEText`) (`self.LText`))
      (`WidgetBlueprintLibrary.SetInputMode_GameAndUIEx` _returnvalue _tutorialwidget)
      (`GameplayStatics.SetGamePaused` true))))

(event `Key|LeftMouseButton` :paused true
  (params (Key :type "Key Structure"))
  (bind _tutorialwidget (`self.TutorialWidget`))
  ;[1 1 1] Exiting
  (:`Pressed`
    (`GameplayStatics.SetGamePaused` false :!label _label)
    (`WidgetBlueprintLibrary.SetInputMode_GameOnly` (`GameplayStatics.GetPlayerController` 0))
    (`Widget.SetVisibility` _tutorialwidget "Collapsed")
    (`Widget.RemoveFromParent` _tutorialwidget)
    (`KismetSystemLibrary.CollectGarbage`)
    (`self.K2_DestroyActor`)))

(event `Key|Gamepad_FaceButton_Bottom` :paused true
  (params (Key :type "Key Structure"))
  ;[1 1 1] Exiting
  (:`Pressed`
    (goto _label)))

(fn `UserConstructionScript`)