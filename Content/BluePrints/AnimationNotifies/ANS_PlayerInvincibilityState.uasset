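; Anim notify state that makes the player invincible for the span it covers on an animation.
; Notify begin casts the mesh owner to BP_MythicismPlayer and sets IsInvincible on its Attributes to true, and notify end sets it back to false.
; Owners that are not BP_MythicismPlayer are left unaffected.
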(fn `Received_NotifyBegin`
  (params (MeshComp :type "SkeletalMeshComponent Object Reference") (Animation :type "AnimSequenceBase Object Reference") (TotalDuration :type "Float (double-precision)"))
  (returns (ReturnValue :type Boolean))
  (bind _asbp_mythicism_player (cast `/Game/BluePrints/MythicismPlayer/BP_MythicismPlayer` (`ActorComponent.GetOwner` MeshComp)))
  (set `CharacterAttributesComponent.isInvincible` true (`MythicismPlayer.attributes` _asbp_mythicism_player))
  (return true))

(fn `Received_NotifyEnd`
  (params (MeshComp :type "SkeletalMeshComponent Object Reference") (Animation :type "AnimSequenceBase Object Reference"))
  (returns (ReturnValue :type Boolean))
  (bind _asbp_mythicism_player (cast `/Game/BluePrints/MythicismPlayer/BP_MythicismPlayer` (`ActorComponent.GetOwner` MeshComp)))
  (set `CharacterAttributesComponent.isInvincible` false (`MythicismPlayer.attributes` _asbp_mythicism_player))
  (return false))