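; Animation notify that plays a footstep sound when triggered during an animation.
; Received_Notify plays Footstep_Cue at the mesh component's world location, scaled by the Volume variable, then returns false.
; Disconnected nodes hold an unused alternative with a random integer switch and five individual footstep sounds, none of which run.
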(fn `Received_Notify`
  (params (MeshComp :type "SkeletalMeshComponent Object Reference") (Animation :type "AnimSequenceBase Object Reference"))
  (returns (ReturnValue :type Boolean))
  (`GameplayStatics.PlaySoundAtLocation` "/Game/Audio/Footsteps/footstep_Cue.footstep_Cue" (`SceneComponent.K2_GetComponentLocation` MeshComp) (struct) (`self.volume`) 1.0 0.0 null null null)
  (return false))