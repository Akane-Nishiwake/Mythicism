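; Anim notify state that shows the player's shield on the back instead of in the hand for part of an animation.
; On begin and every tick it shows BP_MythicismPlayer's BackSocket component and hides ShieldHand, without propagating to children.
; On end it reverses both, putting the shield back in the hand.
; It does nothing when the mesh owner is not BP_MythicismPlayer.
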(fn `Received_NotifyBegin`
  (params (MeshComp :type "SkeletalMeshComponent Object Reference") (Animation :type "AnimSequenceBase Object Reference") (TotalDuration :type "Float (double-precision)"))
  (returns (ReturnValue :type Boolean))
  (bind _asbp_mythicism_player (cast `/Game/BluePrints/MythicismPlayer/BP_MythicismPlayer` (`ActorComponent.GetOwner` MeshComp)))
  (`SceneComponent.SetVisibility` (`/Game/BluePrints/MythicismPlayer/BP_MythicismPlayer.Back Socket` _asbp_mythicism_player) true false)
  (`SceneComponent.SetVisibility` (`MythicismCharacter.shieldHand` _asbp_mythicism_player) false false)
  (return false))

(fn `Received_NotifyEnd`
  (params (MeshComp :type "SkeletalMeshComponent Object Reference") (Animation :type "AnimSequenceBase Object Reference"))
  (returns (ReturnValue :type Boolean))
  (bind _asbp_mythicism_player (cast `/Game/BluePrints/MythicismPlayer/BP_MythicismPlayer` (`ActorComponent.GetOwner` MeshComp)))
  (`SceneComponent.SetVisibility` (`/Game/BluePrints/MythicismPlayer/BP_MythicismPlayer.Back Socket` _asbp_mythicism_player) false false)
  (`SceneComponent.SetVisibility` (`MythicismCharacter.shieldHand` _asbp_mythicism_player) true false)
  (return false))

(fn `Received_NotifyTick`
  (params (MeshComp :type "SkeletalMeshComponent Object Reference") (Animation :type "AnimSequenceBase Object Reference") (FrameDeltaTime :type "Float (double-precision)"))
  (returns (ReturnValue :type Boolean))
  (bind _asbp_mythicism_player (cast `/Game/BluePrints/MythicismPlayer/BP_MythicismPlayer` (`ActorComponent.GetOwner` MeshComp)))
  (`SceneComponent.SetVisibility` (`/Game/BluePrints/MythicismPlayer/BP_MythicismPlayer.Back Socket` _asbp_mythicism_player) true false)
  (`SceneComponent.SetVisibility` (`MythicismCharacter.shieldHand` _asbp_mythicism_player) false false)
  (return false))