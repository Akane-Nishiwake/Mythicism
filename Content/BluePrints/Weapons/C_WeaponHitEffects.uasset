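; Weapon component that provides hit feedback effects: hit stop and a brief light flash.
; The HitStop event waits briefly, then calls ReceiveHitStop on both the enemy and the player with a short duration.
; SpawnLightFlash spawns a small, warm, shadowless point light just above the owning actor and uses its lifespan to remove it almost immediately.
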(event `HitStop`
  (params (Enemy :type "/Game/BluePrints/Enemies/BP_Enemy_1_Character Object Reference") (Player :type "/Game/BluePrints/MythicismPlayer/BP_MythicismPlayer Object Reference"))
  ;[1 1 1] Call hitstop receivers
  (`KismetSystemLibrary.Delay` 0.1)
  (`/Game/BluePrints/Enemies/BP_Enemy_1_Character.ReceiveHitStop` Enemy 0.08)
  (`/Game/BluePrints/MythicismPlayer/BP_MythicismPlayer.ReceiveHitStop` Player 0.08))

(fn `SpawnLightFlash`
  (bind (_returnvalue_location _returnvalue_rotation _returnvalue_scale) (`KismetMathLibrary.BreakTransform` (`Actor.GetTransform` (`self.GetOwner`))))
  (bind _returnvalue (`|SpawnActorFromClass` "/Script/Engine.PointLight" (`KismetMathLibrary.MakeTransform` (+ (* (`KismetMathLibrary.GetUpVector` _returnvalue_rotation) 50.0) _returnvalue_location) _returnvalue_rotation _returnvalue_scale) "Undefined" "OverrideRootScale" null null))
  (bind _pointlightcomponent (`PointLight.PointLightComponent` _returnvalue))
  (`LightComponent.SetIntensity` _pointlightcomponent 800.0)
  (`LocalLightComponent.SetAttenuationRadius` _pointlightcomponent 80.0)
  (`LightComponentBase.SetCastShadows` _pointlightcomponent false)
  (`LightComponent.SetLightColor` _pointlightcomponent (struct :`R` 0.734375 :`G` 0.651017 :`B` 0.590649 :`A` 1.0) true)
  (`Actor.SetLifeSpan` _returnvalue 0.1))