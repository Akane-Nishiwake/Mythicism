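; Anim notify state that opens a melee damage window on the owning character's current weapon during an animation.
; On begin, it casts the mesh owner to MythicismCharacter and enables damage dealing on the valid current weapon, passing the notify's AttackStrength.
; On end, it disables damage dealing on that character's current weapon.
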(fn `Received_NotifyBegin`
  (params (MeshComp :type "SkeletalMeshComponent Object Reference") (Animation :type "AnimSequenceBase Object Reference") (TotalDuration :type "Float (double-precision)"))
  (returns (ReturnValue :type Boolean))
  (bind _asmythicism_character (cast `MythicismCharacter` (`ActorComponent.GetOwner` MeshComp)))
  (bind _returnvalue (`MythicismCharacter.GetCurrentWeapon` _asmythicism_character))
  (if (`KismetSystemLibrary.IsValid` _returnvalue)
    (`Weapon.EnableDealingDamage` _returnvalue (`self.attackStrength`)))
  (return false))

(fn `Received_NotifyEnd`
  (params (MeshComp :type "SkeletalMeshComponent Object Reference") (Animation :type "AnimSequenceBase Object Reference"))
  (returns (ReturnValue :type Boolean))
  (bind _asmythicism_character (cast `MythicismCharacter` (`ActorComponent.GetOwner` MeshComp)))
  (bind _returnvalue (`MythicismCharacter.GetCurrentWeapon` _asmythicism_character))
  (if (`KismetSystemLibrary.IsValid` _returnvalue)
    (`Weapon.DisableDealingDamage` _returnvalue))
  (return false))