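; Animation notify that makes an Enemy cast a fire quick spell when the animation reaches it.
; It casts the mesh owner to Enemy and spawns BP_EnemyQuickSpell_Fire at the current weapon's location, rotated to the pawn's base aim rotation.
; It then calls FireSpell with the mesh component's forward vector as the direction, rather than the aim rotation.
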(fn `Received_Notify`
  (params (MeshComp :type "SkeletalMeshComponent Object Reference") (Animation :type "AnimSequenceBase Object Reference"))
  (returns (ReturnValue :type Boolean))
  (bind _asenemy (cast `Enemy` (`ActorComponent.GetOwner` MeshComp) :!pure true))
  (bind _returnvalue (`|SpawnActorFromClass` "/Game/BluePrints/SpellsAndCurses/EnemySpells/BP_EnemyQuickSpell_Fire.BP_EnemyQuickSpell_Fire_C" (`KismetMathLibrary.ComposeTransforms` (`KismetMathLibrary.Conv_RotatorToTransform` (`Pawn.GetBaseAimRotation` (`PawnMovementComponent.GetPawnOwner` (`Character.CharacterMovement` _asenemy)))) (`KismetMathLibrary.Conv_VectorToTransform` (`Actor.K2_GetActorLocation` (`MythicismCharacter.GetCurrentWeapon` _asenemy)))) "Undefined" "OverrideRootScale" null null))
  (`QuickSpell.FireSpell` _returnvalue (`SceneComponent.GetForwardVector` MeshComp))
  (return false))