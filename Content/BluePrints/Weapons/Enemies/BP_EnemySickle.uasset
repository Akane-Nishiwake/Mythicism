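; Enemy sickle weapon that adds impact feedback when it lands a hit.
; On a weapon hit it disables further damage, then pairs the hit receiver with the parent actor as enemy and player, in either direction.
; For a valid pair, the CWeaponHitEffects component applies hitstop to both characters and spawns a light flash.
; The collider overlap event and construction script are empty.
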(event `self.hitCollider.OnComponentBeginOverlap`
  (params (OverlappedComponent :type "PrimitiveComponent Object Reference") (OtherActor :type "Actor Object Reference") (OtherComp :type "PrimitiveComponent Object Reference") (OtherBodyIndex :type Integer) (bFromSweep :type Boolean) (SweepResult :type "HitResult Structure (by ref)")))

(event `self.OnWeaponHit`
  (params (hitReceiver :type "Actor Object Reference"))
  ;[1 1 1] Hitstop
  (`self.DisableDealingDamage`)
  (bind _asbp_enemy_1_character (cast `/Game/BluePrints/Enemies/BP_Enemy_1_Character` hitReceiver)
    (:`then`
      (bind _asbp_mythicism_player (cast `/Game/BluePrints/MythicismPlayer/BP_MythicismPlayer` (`self.GetParentActor`)))
      (`/Game/BluePrints/Weapons/C_WeaponHitEffects.HitStop` (`self.C_WeaponHitEffects`) _asbp_enemy_1_character _asbp_mythicism_player))
    (:`CastFailed`
      (bind _asbp_mythicism_player_2 (cast `/Game/BluePrints/MythicismPlayer/BP_MythicismPlayer` hitReceiver))
      (bind _asbp_enemy_1_character_2 (cast `/Game/BluePrints/Enemies/BP_Enemy_1_Character` (`self.GetParentActor`)))
      (`/Game/BluePrints/Weapons/C_WeaponHitEffects.HitStop` (`self.C_WeaponHitEffects`) _asbp_enemy_1_character_2 _asbp_mythicism_player_2)))
  (`/Game/BluePrints/Weapons/C_WeaponHitEffects.SpawnLightFlash` (`self.C_WeaponHitEffects`)))

(fn `UserConstructionScript`)