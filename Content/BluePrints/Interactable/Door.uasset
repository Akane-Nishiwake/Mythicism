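; Interactable door that swings open when an in-range player presses Interact, optionally locked behind a key.
; Locked doors check the player's inventory for a matching KeyCode, while a StuckKey code only shows a stuck message.
; Alerts go through the game mode's AlertWidget, naming the required key type when locked, alongside 2D sounds.
; Opening plays a timeline that yaws the root by OpenAngle relative to its starting rotation.
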(event `UnlockedPrompt`
  (bind _asthird_person_game_mode (cast `/Game/BluePrints/ThirdPersonCharacter/ThirdPersonGameMode` (`GameplayStatics.GetGameMode`)))
  (`/Game/BluePrints/UI/PlayerHud/BP_Alert.AppearWithText` (`/Game/BluePrints/ThirdPersonCharacter/ThirdPersonGameMode.AlertWidget` _asthird_person_game_mode) (`self.UnlockedText`))
  (`GameplayStatics.PlaySound2D` "/Game/Audio/DoorSounds/536092__eminyildirim__old-metalic-door-locked_Cue.536092__eminyildirim__old-metalic-door-locked_Cue" 1.0 1.0 0.0 null null))

(event `LockedPrompt`
  (bind _returnvalue (`KismetTextLibrary.Conv_TextToString` (`self.LockedText1`)))
  (bind _asthird_person_game_mode (cast `/Game/BluePrints/ThirdPersonCharacter/ThirdPersonGameMode` (`GameplayStatics.GetGameMode`)))
  (switch `string` (`KismetTextLibrary.Conv_TextToString` (`self.KeyCode`))
    (:`Default`
      (bind _alertwidget (`/Game/BluePrints/ThirdPersonCharacter/ThirdPersonGameMode.AlertWidget` _asthird_person_game_mode))
      (`/Game/BluePrints/UI/PlayerHud/BP_Alert.AppearWithText` _alertwidget (`KismetTextLibrary.Conv_StringToText` (`KismetStringLibrary.Concat_StrStr` _returnvalue "key."))))
    (:`testdoor`
      (`/Game/BluePrints/UI/PlayerHud/BP_Alert.AppearWithText` _alertwidget (`KismetTextLibrary.Conv_StringToText` (`KismetStringLibrary.Concat_StrStr` _returnvalue "golden key."))))
    (:`wizard`
      (`/Game/BluePrints/UI/PlayerHud/BP_Alert.AppearWithText` _alertwidget (`KismetTextLibrary.Conv_StringToText` (`KismetStringLibrary.Concat_StrStr` _returnvalue "wizard's key."))))
    (:`diamond`
      (`/Game/BluePrints/UI/PlayerHud/BP_Alert.AppearWithText` _alertwidget (`KismetTextLibrary.Conv_StringToText` (`KismetStringLibrary.Concat_StrStr` _returnvalue "diamond key."))))
    (:`training`
      (`/Game/BluePrints/UI/PlayerHud/BP_Alert.AppearWithText` _alertwidget (`KismetTextLibrary.Conv_StringToText` (`KismetStringLibrary.Concat_StrStr` _returnvalue "colliseum key."))))
    (:`holy`
      (`/Game/BluePrints/UI/PlayerHud/BP_Alert.AppearWithText` _alertwidget (`KismetTextLibrary.Conv_StringToText` (`KismetStringLibrary.Concat_StrStr` _returnvalue "holy key."))))
    (:`secret`
      (`/Game/BluePrints/UI/PlayerHud/BP_Alert.AppearWithText` _alertwidget (`KismetTextLibrary.Conv_StringToText` (`KismetStringLibrary.Concat_StrStr` _returnvalue "silver key.")))))
  (`GameplayStatics.PlaySound2D` "/Game/Audio/DoorSounds/580442__bennynz__dungeon-lock-2_Cue.580442__bennynz__dungeon-lock-2_Cue" 1.0 1.0 0.0 null null))

(event `self.ReceiveBeginPlay`
  (`parent.ReceiveBeginPlay`)
  (set `self.StartAngle` (.yaw (`SceneComponent.K2_GetComponentRotation` (`self.root`)))))

(event `InputAction|Interact` :consume false
  (params (Key :type "Key Structure"))
  (:`Pressed`
    (if (and (`self.playerInRange`) (not (`self.Opened`)))
      (if (`self.Locked`)
        (if (`KismetTextLibrary.EqualEqual_TextText` (`self.KeyCode`) (`self.stuckKey`))
          (bind _asthird_person_game_mode (cast `/Game/BluePrints/ThirdPersonCharacter/ThirdPersonGameMode` (`GameplayStatics.GetGameMode`)))
          (`/Game/BluePrints/UI/PlayerHud/BP_Alert.AppearWithText` (`/Game/BluePrints/ThirdPersonCharacter/ThirdPersonGameMode.AlertWidget` _asthird_person_game_mode) (`self.StuckText`))
          (else
            (bind _asbp_mythicism_player (cast `/Game/BluePrints/MythicismPlayer/BP_MythicismPlayer` (`GameplayStatics.GetPlayerPawn` 0)))
            (bind _returnvalue (`Inventory.KeyCodeExists` (`/Game/BluePrints/MythicismPlayer/BP_MythicismPlayer.Inventory` _asbp_mythicism_player) (`self.KeyCode`)))
            (if _returnvalue
              (`self.Open`)
              (`self.UnlockedPrompt`)
              (`GameplayStatics.PlaySound2D` "/Game/Audio/DoorSounds/161393__tuben__metal-door-open_Cue.161393__tuben__metal-door-open_Cue" 1.0 1.0 0.0 null null)
              (else
                (`self.LockedPrompt`)))))
        (else
          (`self.Open`)
          (`GameplayStatics.PlaySound2D` "/Game/Audio/DoorSounds/161393__tuben__metal-door-open_Cue.161393__tuben__metal-door-open_Cue" 1.0 1.0 0.0 null null))))))

(event `Open`
  (bind (_direction _currentanglemultiplier) (`Timeline|OpenAnim`)
    (:`Update`
      (`SceneComponent.K2_SetWorldRotation` (`self.root`) (`KismetMathLibrary.MakeRotator` 0.0 0.0 (+ (* (`self.OpenAngle`) _currentanglemultiplier) (`self.StartAngle`))) false false))))

(fn `UserConstructionScript`
  (`parent.UserConstructionScript`))