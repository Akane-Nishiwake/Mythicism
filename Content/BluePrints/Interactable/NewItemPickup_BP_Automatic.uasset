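; Automatic item pickup that grants and equips its item at level start, with no pickup prompt.
; On BeginPlay it destroys itself if the "save1" slot lists any picked-up names; the name comparison is unwired.
; It then runs parent BeginPlay and, after a short delay, records its name on the player and silently adds the item to inventory.
; It equips and highlights the matching weapon, spell or consumable button by Index, then destroys itself.
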(event `self.ReceiveBeginPlay`
  (`|ExecutionSequence`
    (:`then_0`
      (bind _returnvalue (`GameplayStatics.LoadGameFromSlot` "save1"))
      (bind _assave_slot (cast `/Game/BluePrints/SaveSystem/SaveSlot` _returnvalue))
      (for _array_element (`/Game/BluePrints/SaveSystem/SaveSlot.PickupItemNames` _assave_slot)
        (if true
          (`self.K2_DestroyActor`))))
    (:`then_1`
      (`parent.ReceiveBeginPlay`)
      (`KismetSystemLibrary.Delay` 0.2)
      (bind _asbp_mythicism_player (cast `/Game/BluePrints/MythicismPlayer/BP_MythicismPlayer` (`GameplayStatics.GetPlayerCharacter` 0)))
      (`KismetArrayLibrary.Array_Add` (`/Game/BluePrints/MythicismPlayer/BP_MythicismPlayer.GrabbedItemNames` _asbp_mythicism_player) (`KismetStringLibrary.Conv_StringToName` (`KismetSystemLibrary.GetObjectName` self)))
      (set `self.DisplaysGotItemPrompt` false)
      (bind _returnvalue_2 (`self.GetItemData`))
      (bind _asthird_person_game_mode (cast `/Game/BluePrints/ThirdPersonCharacter/ThirdPersonGameMode` (`GameplayStatics.GetGameMode`)))
      (`/Game/BluePrints/GameManager/BP_GameManager.SilentlyAddItemToInventory` (`/Game/BluePrints/ThirdPersonCharacter/ThirdPersonGameMode.GameManager` _asthird_person_game_mode) _returnvalue_2)
      (bind _asthird_person_game_mode_2 (cast `/Game/BluePrints/ThirdPersonCharacter/ThirdPersonGameMode` (`GameplayStatics.GetGameMode`)))
      (cast `WeaponItem` _returnvalue_2
        (:`then`
          (bind _inventorywidget (`/Game/BluePrints/ThirdPersonCharacter/ThirdPersonGameMode.InventoryWidget` _asthird_person_game_mode_2))
          (bind _output (`|GetArrayItem` (`/Game/BluePrints/UI/Inventory/BP_InventoryUI.WeaponButtons` _inventorywidget) (`self.Index`)))
          (`/Game/BluePrints/UI/Inventory/BP_InventoryWeaponUI.Equip` _output)
          (`Widget.SetVisibility` (`/Game/BluePrints/UI/Inventory/BP_InventoryWeaponUI.EquippedHighlight` _output) "SelfHitTestInvisible"))
        (:`CastFailed`
          (cast `SpellItem` _returnvalue_2
            (:`then`
              (bind _output_2 (`|GetArrayItem` (`/Game/BluePrints/UI/Inventory/BP_InventoryUI.SpellButtons` _inventorywidget) (`self.Index`)))
              (`/Game/BluePrints/UI/Inventory/BP_InventorySpellUI.Equip` _output_2)
              (`Widget.SetVisibility` (`/Game/BluePrints/UI/Inventory/BP_InventorySpellUI.EquippedHighlight` _output_2) "SelfHitTestInvisible"))
            (:`CastFailed`
              (bind _asconsumable_item (cast `ConsumableItem` _returnvalue_2))
              (bind _output_3 (`|GetArrayItem` (`/Game/BluePrints/UI/Inventory/BP_InventoryUI.ConsumableButtons` _inventorywidget) (`self.Index`)))
              (`/Game/BluePrints/UI/Inventory/BP_InventoryConsumableUI.Equip` _output_3)
              (`Widget.SetVisibility` (`/Game/BluePrints/UI/Inventory/BP_InventoryConsumableUI.EquippedHighlight` _output_3) "SelfHitTestInvisible")))))
      (`self.K2_DestroyActor`))))

(fn `UserConstructionScript`
  (`parent.UserConstructionScript`))