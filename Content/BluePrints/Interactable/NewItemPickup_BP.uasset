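; Interactable item pickup that goes to the player when Interact is pressed in range, then destroys itself.
; It casts the item data to weapon, spell, key or consumable to update the Inventory component and inventory UI, though consumables only reach the UI.
; An optional flag shows the got-item prompt with a sound.
; Grabbed pickups record their object name on the player, and BeginPlay destroys any whose name is in the save slot.
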(event `DisplayGotItemPrompt`
  (bind _returnvalue (`self.GetItemData`))
  (bind _asthird_person_game_mode (cast `/Game/BluePrints/ThirdPersonCharacter/ThirdPersonGameMode` (`GameplayStatics.GetGameMode`)))
  (`/Game/BluePrints/UI/PlayerHud/BP_GotItem.AppearWithItem` (`/Game/BluePrints/ThirdPersonCharacter/ThirdPersonGameMode.GotItemWidget` _asthird_person_game_mode) _returnvalue))

(event `AddToInventory`
  (`self.InteractFunction`)
  (bind _returnvalue (`self.GetItemData`))
  (bind _returnvalue_2 (`GameplayStatics.GetActorOfClass` "/Game/BluePrints/MythicismPlayer/BP_MythicismPlayer.BP_MythicismPlayer_C"))
  (bind _asweapon_item (cast `WeaponItem` _returnvalue)
    (:`then`
      (bind _returnvalue_3 (`self.GetComponentByClass` _returnvalue_2 "/Script/Mythicism.Inventory"))
      (`Inventory.AddWeapon` _returnvalue_3 _asweapon_item)
      (bind _asthird_person_game_mode (cast `/Game/BluePrints/ThirdPersonCharacter/ThirdPersonGameMode` (`GameplayStatics.GetGameMode`)))
      (`/Game/BluePrints/UI/Inventory/BP_InventoryUI.AddWeaponToUI` (`/Game/BluePrints/ThirdPersonCharacter/ThirdPersonGameMode.InventoryWidget` _asthird_person_game_mode) _asweapon_item)
      (if (`self.DisplaysGotItemPrompt`)
        (`self.DisplayGotItemPrompt`)
        (`GameplayStatics.PlaySound2D` "/Game/Audio/Impact/Explosion02.Explosion02" 1.0 1.0 0.0 null null :!label _label)))
    (:`CastFailed`
      (bind _asspell_item (cast `SpellItem` _returnvalue)
        (:`then`
          (`Inventory.AddSpell` _returnvalue_3 _asspell_item)
          (bind _asthird_person_game_mode_2 (cast `/Game/BluePrints/ThirdPersonCharacter/ThirdPersonGameMode` (`GameplayStatics.GetGameMode`)))
          (`/Game/BluePrints/UI/Inventory/BP_InventoryUI.AddSpellToUI` (`/Game/BluePrints/ThirdPersonCharacter/ThirdPersonGameMode.InventoryWidget` _asthird_person_game_mode_2) _asspell_item)
          (if (`self.DisplaysGotItemPrompt`)
            (`self.DisplayGotItemPrompt`)
            (goto _label)
            (else
              _)))
        (:`CastFailed`
          (bind _askey_item (cast `KeyItem` _returnvalue)
            (:`then`
              (`Inventory.AddKey` _returnvalue_3 _askey_item)
              (bind _asthird_person_game_mode_3 (cast `/Game/BluePrints/ThirdPersonCharacter/ThirdPersonGameMode` (`GameplayStatics.GetGameMode`)))
              (`/Game/BluePrints/UI/Inventory/BP_InventoryUI.AddKeyToUI` (`/Game/BluePrints/ThirdPersonCharacter/ThirdPersonGameMode.InventoryWidget` _asthird_person_game_mode_3) _askey_item)
              (if (`self.DisplaysGotItemPrompt`)
                (`self.DisplayGotItemPrompt`)
                (goto _label)
                (else
                  _)))
            (:`CastFailed`
              (bind _asconsumable_item (cast `ConsumableItem` _returnvalue))
              (bind _asthird_person_game_mode_4 (cast `/Game/BluePrints/ThirdPersonCharacter/ThirdPersonGameMode` (`GameplayStatics.GetGameMode`)))
              (`/Game/BluePrints/UI/Inventory/BP_InventoryUI.AddConsumableToUI` (`/Game/BluePrints/ThirdPersonCharacter/ThirdPersonGameMode.InventoryWidget` _asthird_person_game_mode_4) _asconsumable_item)
              (if (`self.DisplaysGotItemPrompt`)
                (`self.DisplayGotItemPrompt`)
                (goto _label)
                (else
                  _))))))))
  (`self.K2_DestroyActor`))

(event `InputAction|Interact` :consume false
  (params (Key :type "Key Structure"))
  (:`Pressed`
    (if (`self.playerInRange`)
      (bind _asbp_mythicism_player (cast `/Game/BluePrints/MythicismPlayer/BP_MythicismPlayer` (`GameplayStatics.GetPlayerCharacter` 0)))
      (`KismetArrayLibrary.Array_Add` (`/Game/BluePrints/MythicismPlayer/BP_MythicismPlayer.GrabbedItemNames` _asbp_mythicism_player) (`KismetStringLibrary.Conv_StringToName` (`KismetSystemLibrary.GetObjectName` self)))
      (`self.AddToInventory`))))

(event `self.ReceiveBeginPlay`
  (bind _returnvalue (`GameplayStatics.LoadGameFromSlot` "save1"))
  (bind _assave_slot (cast `/Game/BluePrints/SaveSystem/SaveSlot` _returnvalue))
  (for _array_element (`/Game/BluePrints/SaveSystem/SaveSlot.PickupItemNames` _assave_slot)
    (if (== _array_element (`KismetStringLibrary.Conv_StringToName` (`KismetSystemLibrary.GetObjectName` self)))
      (`self.K2_DestroyActor`))))

(fn `UserConstructionScript`)