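; BP_WinPortal is an interactable portal actor that ends the game with a win screen when overlapped.
; Any actor overlap starts a short delay, then a camera and audio fade-out that holds.
; After the fade it creates the BP_WinScreen widget, shows the mouse cursor and switches to UI-only input.
; The Interact input checks PlayerInRange but triggers nothing.
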(event `self.ReceiveActorBeginOverlap`
  (params (OtherActor :type "Actor Object Reference"))
  (bind _returnvalue (`GameplayStatics.GetPlayerController` 0))
  (`KismetSystemLibrary.Delay` 2.0)
  (`PlayerCameraManager.StartCameraFade` :`self` (`PlayerController.PlayerCameraManager` (`GameplayStatics.GetPlayerController` 0)) :`ToAlpha` 1.0 :`Duration` 2.0 :`bShouldFadeAudio` true :`bHoldWhenFinished` true)
  (`KismetSystemLibrary.Delay` 2.0)
  (bind _returnvalue_2 (`|CreateWidget` "/Game/BluePrints/UI/WinLose/BP_WinScreen.BP_WinScreen_C"))
  (`UserWidget.AddToViewport` _returnvalue_2 0)
  (set `PlayerController.bShowMouseCursor` true _returnvalue)
  (`WidgetBlueprintLibrary.SetInputMode_UIOnlyEx` _returnvalue null))

(event `InputAction|Interact` :consume false
  (params (Key :type "Key Structure"))
  (:`Pressed`
    (if (`self.playerInRange`)
      _)))

(fn `UserConstructionScript`)